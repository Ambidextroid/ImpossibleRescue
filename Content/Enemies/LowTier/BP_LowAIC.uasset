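; AI controller for low-tier enemies that turns to face the player and fires projectiles at them.
; On possession it caches the BP_LowEnemy pawn, then each tick rotates that enemy's model toward the player while it has line of sight.
; Each PawnSensing sighting of a Player-tagged pawn spawns a projectile from the model aimed at the player, so fire rate follows the sensing events.
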(event OnSeePawn(PawnSensing)
  (params (Pawn :type Pawn%20Object%20Reference))
  (bind _enemyreference (Variables|Default|GetEnemyReference))
  (bind _modelroot (Variables|/Game/Enemies/LowTier/BP_LowEnemy.BP_LowEnemy_C|GetModelRoot _enemyreference))
  (bind _returnvalue (Transformation|GetWorldLocation _modelroot))
  ;[1 1 1] Shoot periodically when enemy senses player
  (if (Actor|ActorHasTag Pawn "Player")
    (Game|SpawnActorfromClass "/Game/Enemies/LowTier/BP_LowEnemyProjectile.BP_LowEnemyProjectile_C" (Math|Transform|MakeTransform _returnvalue (Math|Conversions|RotationFromXVector (Math|Vector|GetUnitDirection(Vector) _returnvalue (Transformation|GetActorLocation (Game|Player|GetPlayerPawn 0)))) "0.500000,0.100000,0.100000") "Undefined" 0 0)))

(event EventBeginPlay)

(event EventTick
  (params (DeltaSeconds :type Float%20%28single-precision%29))
  ;[1 1 1] Face player when line of sight
  (if (Controller|LineOfSightTo (Game|Player|GetPlayerPawn 0) "0, 0, 0" false)
    (Transformation|SetWorldRotation (Variables|/Game/Enemies/LowTier/BP_LowEnemy.BP_LowEnemy_C|GetModelRoot (Variables|Default|GetEnemyReference)) (Math|Conversions|RotationFromXVector (Math|Vector|GetUnitDirection(Vector) (Transformation|GetWorldLocation (Variables|/Script/Engine.Actor|GetRootComponent (Variables|Default|GetEnemyReference))) (Transformation|GetActorLocation (Game|Player|GetPlayerPawn 0)))) false false)))

(event EventPossess
  (params (PossessedPawn :type Pawn%20Object%20Reference))
  (bind _asbp_low_enemy (Utilities|Casting|CastToBP_LowEnemy PossessedPawn))
  (Variables|Default|SetEnemyReference _asbp_low_enemy))

(fn ConstructionScript)