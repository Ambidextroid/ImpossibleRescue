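; Enemy laser turret that tracks the player, locks its aim, then fires a damaging beam.
; A self-repeating delay cycle moves it through aim, warning and fire phases, with a start offset.
; A looping timeline eases an aim target toward the player and colors the sight green or orange by phase.
; Horizontal line traces place the sight, beam and sparks, and apply delta-time-scaled damage along the locked line.
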(event Custom|FireCycle
  (bind _laser (Variables|Default|GetLaser))
  (bind _aimdirection (Variables|Default|GetAimDIrection))
  (bind _returnvalue (Transformation|GetWorldLocation _aimdirection))
  (bind (_x _y _z) (Math|Vector|BreakVector _returnvalue))
  ;[1 1 1] Laser firing cycle
  (Variables|Default|SetAiming true)
  (Utilities|FlowControl|Delay (Variables|Default|GetTimeAiming))
  (Variables|Default|SetAiming false)
  ;;[1 1 1] Cast ray in direction of player (for laser VFX)
  (Variables|Default|SetTarget (Transformation|GetWorldLocation (Variables|Default|GetAimTarget)))
  (Utilities|FlowControl|Delay (Variables|Default|GetTimeBeforeFiring))
  (bind _outhit (Collision|LineTraceByChannel (Math|Vector|MakeVector _x _y _z) (Math|Vector|MakeVector (.x (+ (Math|Vector|MakeVector _x _y 0.0) (* (Math|Vector|GetUnitDirection(Vector) (Math|Vector|MakeVector _x _y 0.0) (Math|Vector|MakeVector (.X (Math|Vector|BreakVector (Variables|Default|GetTarget))) (.Y (Math|Vector|BreakVector (Variables|Default|GetTarget))) 0.0)) 5e+03))) (.y (+ (Math|Vector|MakeVector _x _y 0.0) (* (Math|Vector|GetUnitDirection(Vector) (Math|Vector|MakeVector _x _y 0.0) (Math|Vector|MakeVector (.X (Math|Vector|BreakVector (Variables|Default|GetTarget))) (.Y (Math|Vector|BreakVector (Variables|Default|GetTarget))) 0.0)) 5e+03))) _z) "TraceTypeQuery4" false 0 "None"))
  ;;[1 1 1] Set laser beam endpoint and activate spark effects
  (Effects|Components|ParticleSystem|SetVectorParameter _laser "LaserEnd" (- (.location _outhit) (Transformation|GetWorldLocation _laser)))
  (Transformation|SetWorldLocationAndRotation (Variables|Default|GetLaserSparks) (.location _outhit) (Math|Conversions|RotationFromXVector (.normal _outhit)) false false)
  (Components|Activation|Activate (Variables|Default|GetLaserSparks) false)
  (Variables|Default|SetFiring true)
  (Utilities|FlowControl|Delay (Variables|Default|GetTimeFiring))
  (Variables|Default|SetFiring false)
  (Components|Activation|Deactivate (Variables|Default|GetLaserSparks))
  (Effects|Components|ParticleSystem|SetVectorParameter (Variables|Default|GetLaser) "LaserEnd" "0, 0, 0")
  (CallFunction|FireCycle))

(event EventBeginPlay
  (bind _aimdirection (Variables|Default|GetAimDIrection))
  (bind _target (Variables|Default|GetTarget))
  (bind _aimtarget (Variables|Default|GetAimTarget))
  (bind _aimdirection_2 (Variables|Default|GetAimDIrection))
  (bind _aimtarget_2 (Variables|Default|GetAimTarget))
  (bind _aimdirection_3 (Variables|Default|GetAimDIrection))
  (bind _aimdirection_4 (Variables|Default|GetAimDIrection))
  (bind _returnvalue (Transformation|GetWorldLocation _aimtarget))
  (bind _returnvalue_2 (Transformation|GetWorldLocation _aimdirection))
  (bind _returnvalue_3 (Transformation|GetWorldLocation _aimdirection_2))
  (bind _returnvalue_4 (Transformation|GetWorldLocation _aimtarget_2))
  (bind _returnvalue_5 (Transformation|GetWorldLocation _aimdirection_3))
  (bind _returnvalue_6 (Transformation|GetWorldLocation _aimdirection_4))
  (bind (_x _y) (Math|Vector|BreakVector _target))
  (bind (_x_2 _y_2) (Math|Vector|BreakVector _returnvalue_4))
  (bind (_x_3 _y_3 _z) (Math|Vector|BreakVector _returnvalue_6))
  (bind (_x_4 _y_4 _z_2) (Math|Vector|BreakVector _returnvalue_5))
  (bind (_x_5 _y_5 _z_3) (Math|Vector|BreakVector _returnvalue_3))
  (bind _returnvalue_7 (Math|Vector|GetUnitDirection(Vector) (Math|Vector|MakeVector (.x _returnvalue_2) (.y _returnvalue_2) 0.0) (Math|Vector|MakeVector _x_2 _y_2 0.0)))
  (bind _returnvalue_8 (Math|Vector|GetUnitDirection(Vector) (Math|Vector|MakeVector _x_4 _y_4 0.0) (Math|Vector|MakeVector _x _y 0.0)))
  (bind _returnvalue_9 (* _returnvalue_7 5e+03))
  (bind _returnvalue_10 (* _returnvalue_8 5e+03))
  (bind _returnvalue_11 (+ (Math|Vector|MakeVector _x_5 _y_5 0.0) _returnvalue_9))
  (bind _returnvalue_12 (+ (Math|Vector|MakeVector _x_4 _y_4 0.0) _returnvalue_10))
  (Utilities|FlowControl|Sequence
    (:then_0
      (Components|Activation|Deactivate (Variables|Default|GetLaserSparks))
      (bind _asbp_player (Utilities|Casting|CastToBP_Player (Game|Player|GetPlayerPawn 0)))
      (Variables|Default|SetPlayerReference _asbp_player)
      (Variables|Default|SetAiming true)
      (Utilities|FlowControl|Delay (Variables|Default|GetCycleTimeOffset))
      (CallFunction|FireCycle))
    (:then_1
      (Timeline|Looping Play
        (:Update
          (if (Variables|Default|GetAiming)
            ;[1 1 1] Laser sight parameters
            (Effects|Components|ParticleSystem|SetColorParameter (Variables|Default|GetSight) "SightColour" "(R=0.000000,G=1.000000,B=0.023420,A=1.000000)")
            ;[1 1 1] Aim at player
            ;;[1 1 1] Update AImTarget position to smoothly follow player
            (Transformation|SetWorldLocation (Variables|Default|GetAimTarget) (+ (Transformation|GetWorldLocation (Variables|Default|GetAimTarget)) (* (- (Transformation|GetWorldLocation (Variables|/Script/Engine.Actor|GetRootComponent (Variables|Default|GetPlayerReference))) (Transformation|GetWorldLocation (Variables|Default|GetAimTarget))) (Variables|Default|GetAimSpeed))) false false)
            ;;[1 1 1] Rotate turret towards AimTarget
            (Transformation|SetWorldRotation (Variables|Default|GetAimDIrection) (Math|Conversions|RotationFromXVector (Math|Vector|GetUnitDirection(Vector) (Math|Vector|MakeVector (.x _returnvalue_2) (.y _returnvalue_2) 0.0) (Math|Vector|MakeVector (.x _returnvalue) (.y _returnvalue) 0.0))) false false)
            ;;[1 1 1] Aim laser sight in direction of AimTarget
            (bind _outhit (Collision|LineTraceByChannel (Math|Vector|MakeVector _x_5 _y_5 _z_3) (Math|Vector|MakeVector (.x _returnvalue_11) (.y _returnvalue_11) _z_3) "TraceTypeQuery2" false 0 "None" true "(R=0.000000,G=0.034457,B=1.000000,A=1.000000)" "(R=1.000000,G=0.718554,B=0.099455,A=1.000000)" :!label _label))
            (Effects|Components|ParticleSystem|SetVectorParameter (Variables|Default|GetSight) "SightEnd" (- (.location _outhit) (Transformation|GetWorldLocation (Variables|Default|GetSight))))
            (elif (Variables|Default|GetFiring)
              (Effects|Components|ParticleSystem|SetVectorParameter (Variables|Default|GetSight) "SightEnd" "0, 0, 0")
              ;[1 1 1] Cast ray to check if player is hit by laser
              (bind _outhit_2 (Collision|LineTraceByChannel (Math|Vector|MakeVector _x_3 _y_3 _z) (Math|Vector|MakeVector (.x _returnvalue_12) (.y _returnvalue_12) _z) "TraceTypeQuery5" false 0 "None" true "(R=1.000000,G=0.251666,B=0.890440,A=1.000000)" "(R=0.001031,G=1.000000,B=0.809745,A=1.000000)"))
              (Utilities|IsValid (.hitactor _outhit_2)
                (:Is%20Valid
                  (Game|Damage|ApplyDamage (.hitactor _outhit_2) (* (Utilities|Time|GetWorldDeltaSeconds) (Variables|Default|GetBaseDamage)) 0 0)))
              (else
                (Effects|Components|ParticleSystem|SetColorParameter (Variables|Default|GetSight) "SightColour" "(R=1.000000,G=0.507393,B=0.000000,A=1.000000)")
                (goto _label)))))))))

(fn ConstructionScript)