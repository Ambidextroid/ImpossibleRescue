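; BP_HighEnemy_Act2 is an Act 2 high-tier enemy Blueprint that builds on a parent class for its behavior.
; On BeginPlay it runs the parent logic, registers its StaticMesh as the ActiveMesh, and hides that mesh if the enemy is not Activated.
; Its Teleportin event calls BaseTeleport, and the construction script only calls the parent.
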(event EventBeginPlay
  (|CallParentFunction)
  (Variables|Default|SetActiveMesh (Variables|Default|GetStaticMesh))
  (if (not (Variables|Default|GetActivated))
    (Rendering|SetVisibility (Variables|Default|GetStaticMesh) false false)))

(event Collision|EventActorBeginOverlap
  (params (OtherActor :type Actor%20Object%20Reference))
  (|CallParentFunction OtherActor) ; This node is disabled and will not be called.\nDrag off pins to build functionality.
)

(event EventTick
  (params (DeltaSeconds :type Float%20%28single-precision%29))
  (|CallParentFunction DeltaSeconds) ; This node is disabled and will not be called.\nDrag off pins to build functionality.
)

(event EventTeleportin
  (CallFunction|BaseTeleport))

(fn ConstructionScript
  (|CallParentFunction))