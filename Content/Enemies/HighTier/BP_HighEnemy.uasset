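; BP_HighEnemy is a high-tier enemy Blueprint that hides its model until it materializes with a teleport-in effect.
; BeginPlay hides the Model if the enemy is not Activated.
; The Teleportin event shows the Model, caches its materials and swaps every slot to a teleport material.
; A timeline drives that material's Radius parameter, scaled by the mesh's bounding sphere, then restores the original materials when finished.
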(event EventBeginPlay
  (|CallParentFunction)
  (if (not (Variables|Default|GetActivated))
    (Rendering|SetVisibility (Variables|Default|GetModel) false false)))

(event Collision|EventActorBeginOverlap
  (params (OtherActor :type Actor%20Object%20Reference))
  (|CallParentFunction OtherActor) ; This node is disabled and will not be called.\nDrag off pins to build functionality.
)

(event EventTick
  (params (DeltaSeconds :type Float%20%28single-precision%29))
  (|CallParentFunction DeltaSeconds) ; This node is disabled and will not be called.\nDrag off pins to build functionality.
)

(event EventTeleportin
  (Rendering|SetVisibility (Variables|Default|GetModel) true false)
  (bind _output_get (Variables|Default|SetOriginalMaterials (Rendering|Material|GetMaterials (Variables|Default|GetModel))))
  (for (_ _array_index) _output_get
    (Rendering|Material|SetMaterial (Variables|Default|GetModel) _array_index "/Game/Materials/Test/Mat_Teleport_Inst.Mat_Teleport_Inst"))
  (bind _radius (Timeline|Timeline_0_0 Play)
    (:Update
      (Rendering|Material|SetScalarParameterValueonMaterials (Variables|Default|GetModel) "Radius" (* _radius (.SphereRadius (Collision|GetComponentBounds (Variables|Default|GetModel))))))
    (:Finished
      (for (_array_element _array_index_2) (Variables|Default|GetOriginalMaterials)
        (Rendering|Material|SetMaterial (Variables|Default|GetModel) _array_index_2 _array_element)))))

(fn ConstructionScript
  (|CallParentFunction))