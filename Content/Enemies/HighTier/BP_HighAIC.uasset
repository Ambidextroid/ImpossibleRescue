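; AI controller for BP_HighEnemy that wanders the navmesh and fires bursts at the player while the enemy is activated.
; MoveCycle starts on BeginPlay and chains moves to random nearby points, repeating on success or failure.
; Tick turns the model toward a visible player and triggers Shoot, throttled by FireDelay.
; Shoot spawns three staggered projectiles, each aimed at the player's position, using BurstDelay timing.
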(event Custom|MoveCycle
  ;[1 1 1] Immediately move to random location and repeat
  (if (Variables|/Game/Enemies/BP_EnemyBase.BP_EnemyBase_C|GetActivated (Variables|Default|GetEnemyReference))
    (AI|AIMoveTo 0 (.RandomLocation (Class|NavigationSystemV1|GetRandomPointinNavigableRadius (Transformation|GetWorldLocation (Variables|/Script/Engine.Actor|GetRootComponent (Variables|Default|GetEnemyReference))) 5e+02 0 0)) 0 5.0 false
      (:OnSuccess
        _)
      (:OnFail
        _))
    (CallFunction|MoveCycle)))

(event Custom|Shoot
  (bind _enemyreference (Variables|Default|GetEnemyReference))
  (bind _rootcomponent (Variables|/Script/Engine.Actor|GetRootComponent _enemyreference))
  (bind _returnvalue (Transformation|GetWorldLocation _rootcomponent))
  ;[1 1 1] Shoot periodically when enemy senses player
  (Utilities|FlowControl|Sequence
    (:then_0
      _)
    (:then_1
      (Utilities|FlowControl|Delay (Variables|Default|GetBurstDelay)))
    (:then_2
      (Utilities|FlowControl|Delay (* (Variables|Default|GetBurstDelay) 2.0))))
  (Game|SpawnActorfromClass "/Game/Enemies/HighTier/BP_HighEnemyProjectile.BP_HighEnemyProjectile_C" (Math|Transform|MakeTransform _returnvalue (Math|Conversions|RotationFromXVector (Math|Vector|GetUnitDirection(Vector) _returnvalue (Transformation|GetActorLocation (Game|Player|GetPlayerPawn 0)))) "0.200000,0.100000,0.100000") "Undefined" 0 0))

(event EventBeginPlay
  ;[1 1 1] Immediately move to random location and repeat
  (CallFunction|MoveCycle))

(event EventTick
  (params (DeltaSeconds :type Float%20%28single-precision%29))
  ;[1 1 1] Face player when line of sight
  (if (Variables|/Game/Enemies/BP_EnemyBase.BP_EnemyBase_C|GetActivated (Variables|Default|GetEnemyReference))
    (if (Controller|LineOfSightTo (Game|Player|GetPlayerPawn 0) "0, 0, 0" false)
      (Transformation|SetWorldRotation (Variables|/Game/Enemies/HighTier/BP_HighEnemy.BP_HighEnemy_C|GetModelRoot (Variables|Default|GetEnemyReference)) (Math|Conversions|RotationFromXVector (Math|Vector|GetUnitDirection(Vector) (Transformation|GetWorldLocation (Variables|/Script/Engine.Actor|GetRootComponent (Variables|Default|GetEnemyReference))) (Transformation|GetActorLocation (Game|Player|GetPlayerPawn 0)))) false false)
      ;[1 1 1] Shooting timing
      (if (not (Variables|Default|GetShooting))
        (Variables|Default|SetShooting true)
        (CallFunction|Shoot)
        (Utilities|FlowControl|Delay (Variables|Default|GetFireDelay))
        (Variables|Default|SetShooting false)))))

(event EventPossess
  (params (PossessedPawn :type Pawn%20Object%20Reference))
  (bind _asbp_high_enemy (Utilities|Casting|CastToBP_HighEnemy PossessedPawn))
  (Variables|Default|SetEnemyReference _asbp_high_enemy))

(fn ConstructionScript)