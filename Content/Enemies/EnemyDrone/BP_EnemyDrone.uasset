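; BP_EnemyDrone is an AI-controlled enemy drone that shoots projectiles at the player.
; On BeginPlay it hands its behavior tree to AIC_Enemy and starts the Shooting timeline.
; Each Shoot event on that timeline checks the HasLineOfSight blackboard key before firing.
; When true, it spawns a stretched BP_EnemyProjectile at the Cube component, aimed at the player, and snaps the capsule's rotation to the same direction.
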(event EventBeginPlay
  (bind _returnvalue (Game|Player|GetPlayerPawn 0))
  (bind _cube (Variables|Default|GetCube))
  (bind _returnvalue_2 (Transformation|GetActorLocation _returnvalue))
  (bind _returnvalue_3 (Transformation|GetWorldLocation _cube))
  (bind _returnvalue_4 (Math|Vector|GetUnitDirection(Vector) _returnvalue_3 _returnvalue_2))
  (bind _returnvalue_5 (Math|Conversions|RotationFromXVector _returnvalue_4))
  (bind _asaic_enemy (Utilities|Casting|CastToAIC_Enemy (AI|GetAIController self)))
  (Default|SetupAIC _asaic_enemy (Variables|Default|GetBT))
  (Timeline|Shooting Play
    (:Shoot
      (if (ScalableFloat|GetValueasBool (AI|GetBlackboard self) (Utilities|Name|MakeLiteralName "HasLineOfSight"))
        (Game|SpawnActorfromClass "/Game/Enemies/BP_EnemyProjectile.BP_EnemyProjectile_C" (Math|Transform|MakeTransform _returnvalue_3 _returnvalue_5 "0.500000,0.100000,0.100000") "Undefined" 0 0)
        (Transformation|SetWorldRotation (Variables|Default|GetCapsuleComponent) _returnvalue_5 false false)))))

(event Collision|EventActorBeginOverlap
  (params (OtherActor :type Actor%20Object%20Reference))
  (|CallParentFunction OtherActor) ; This node is disabled and will not be called.\nDrag off pins to build functionality.
)

(fn ConstructionScript
  (|CallParentFunction))