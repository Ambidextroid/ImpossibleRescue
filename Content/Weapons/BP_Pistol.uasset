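; BP_Pistol is a pistol Blueprint that spawns projectiles when its trigger is pulled.
; A pull with ammo left and Cocked set restarts the PistolFireRate timeline, whose Fire event spawns a scaled BP_Projectile at the Arrow component and decrements Ammo.
; Releasing the trigger stops the timeline and sets Cocked, which this graph never clears.
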(event EventBeginPlay
  (|CallParentFunction) ; This node is disabled and will not be called.\nDrag off pins to build functionality.
)

(event Collision|EventActorBeginOverlap
  (params (OtherActor :type Actor%20Object%20Reference))
  (|CallParentFunction OtherActor) ; This node is disabled and will not be called.\nDrag off pins to build functionality.
)

(event EventTick
  (params (DeltaSeconds :type Float%20%28single-precision%29))
  (|CallParentFunction DeltaSeconds) ; This node is disabled and will not be called.\nDrag off pins to build functionality.
)

(event EventOnTriggerPull
  (bind _arrow (Variables|Default|GetArrow))
  (bind _returnvalue (Transformation|GetWorldTransform _arrow))
  ;[1 1 1] Fire projectile
  (if (> (Variables|Default|GetAmmo) 0)
    (if (Variables|Default|GetCocked)
      (Timeline|PistolFireRate PlayFromStart
        (:Fire
          (Game|SpawnActorfromClass "/Game/PlayerCharacter/Projectile/BP_Projectile.BP_Projectile_C" (Math|Transform|MakeTransform (.location _returnvalue) (.rotation _returnvalue) "0.500000,0.100000,0.100000") "Undefined" 0 0)
          (Math|Integer|DecrementInt (Variables|Default|GetAmmo)))))))

(event EventOnTriggerRelease
  (bind _arrow (Variables|Default|GetArrow))
  (bind _returnvalue (Transformation|GetWorldTransform _arrow))
  ;[1 1 1] Fire projectile
  (Variables|Default|SetCocked true)
  (Timeline|PistolFireRate Stop
    (:Fire
      (Game|SpawnActorfromClass "/Game/PlayerCharacter/Projectile/BP_Projectile.BP_Projectile_C" (Math|Transform|MakeTransform (.location _returnvalue) (.rotation _returnvalue) "0.500000,0.100000,0.100000") "Undefined" 0 0)
      (Math|Integer|DecrementInt (Variables|Default|GetAmmo)))))

(fn ConstructionScript
  (|CallParentFunction))