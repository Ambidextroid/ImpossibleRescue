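; BP_BasePickup is a base actor for pickups that fly to the player and get collected.
; On BeginPlay it caches the player and its own starting location.
; When the model overlaps a component tagged PickupCollider, the ItemZoom timeline lerps the item from that start to the player's current location.
; When the timeline finishes, it calls the empty PickedUp event and destroys the actor.
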(event OnComponentBeginOverlap(Model)
  (params (OverlappedComponent :type Primitive%20Component%20Object%20Reference) (OtherActor :type Actor%20Object%20Reference) (OtherComp :type Primitive%20Component%20Object%20Reference) (OtherBodyIndex :type Integer) (bFromSweep :type Boolean) (SweepResult :type Hit%20Result%20Structure%20%28by%20ref%29))
  ;[1 1 1] Overlap player collision box
  (if (Components|ComponentHasTag OtherComp "PickupCollider")
    ;[1 1 1] Zoom towards player
    (bind _itemzoom (Timeline|ItemZoom Play)
      (:Update
        (Transformation|SetWorldLocation (Variables|Default|GetDefaultSceneRoot) (Math|Vector|Lerp(Vector) (Variables|Default|GetItemPos) (Transformation|GetWorldLocation (Variables|/Script/Engine.Actor|GetRootComponent (Variables|Default|GetPlayerReference))) _itemzoom) false false))
      (:Finished
        (CallFunction|PickedUp)
        (Actor|DestroyActor)))))

(event Custom|PickedUp
  ;[1 1 1] Zoom towards player
)

(event EventBeginPlay
  (bind _asbp_player (Utilities|Casting|CastToBP_Player (Game|Player|GetPlayerPawn 0)))
  (Variables|Default|SetPlayerReference _asbp_player)
  (Variables|Default|SetItemPos (Transformation|GetWorldLocation (Variables|Default|GetDefaultSceneRoot))))

(fn ConstructionScript)