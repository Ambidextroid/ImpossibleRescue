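; Deprecated ACT2 player projectile Blueprint that damages what it hits, built on a parent class.
; CheckForTarget skips collisions with the deprecated player class via ShouldIgnoreCollision.
; Otherwise it sends the damage through the ProjectileCollisionMessage interface call on the target, then destroys itself.
; The event graph holds only disabled default events, and the construction script just calls the parent.
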(event EventBeginPlay
  (|CallParentFunction) ; This node is disabled and will not be called.\nDrag off pins to build functionality.
)

(event Collision|EventActorBeginOverlap
  (params (OtherActor :type Actor%20Object%20Reference))
  (|CallParentFunction OtherActor) ; This node is disabled and will not be called.\nDrag off pins to build functionality.
)

(event EventTick
  (params (DeltaSeconds :type Float%20%28single-precision%29))
  (|CallParentFunction DeltaSeconds) ; This node is disabled and will not be called.\nDrag off pins to build functionality.
)

(fn ConstructionScript
  (|CallParentFunction))

(fn CheckforTarget
  (params (Collision%20Target :type Actor%20Object%20Reference))
  ;[1 1 1] Check whether collision should be ignored
  (bind _shouldignore (CallFunction|ShouldIgnoreCollision Collision%20Target "/Game/ACT2_OLD/Blueprints/Player/DEPR_ACT2_Player_BP.DEPR_ACT2_Player_BP_C"))
  (if (not _shouldignore)
    ;[1 1 1] Attempt interface function on target, then destroy this projectile
    (Class|DEPRACT2DamageInterface|ProjectileCollision(Message) Collision%20Target (Variables|Default|GetDamage))
    (Actor|DestroyActor)))