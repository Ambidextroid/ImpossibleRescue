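; Deprecated ACT2 health pickup Blueprint that offers health to the player.
; It overrides two pickup functions: CanPickup allows collection only while the player's health is below maximum, and OnPickup sends HealthValue to the player through HealthPickupMessage.
; The event graph holds only disabled default events, and the construction script just calls its parent.
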(event EventBeginPlay
  (|CallParentFunction) ; This node is disabled and will not be called.\nDrag off pins to build functionality.
)

(event EventTick
  (params (DeltaSeconds :type Float%20%28single-precision%29))
  (|CallParentFunction DeltaSeconds) ; This node is disabled and will not be called.\nDrag off pins to build functionality.
)

(fn ConstructionScript
  (|CallParentFunction))

(fn OnPickup
  (Class|DEPRACT2PickupInterface|HealthPickup(Message) (Variables|Default|GetPlayer) (Variables|Default|GetHealthValue)))

(fn CanPickup
  (bind _player (Variables|Default|GetPlayer))
  (return (< (Variables|/Game/ACT2_OLD/Blueprints/Player/DEPR_ACT2_Player_BP.DEPR_ACT2_Player_BP_C|GetHealth _player) (Variables|/Game/ACT2_OLD/Blueprints/Player/DEPR_ACT2_Player_BP.DEPR_ACT2_Player_BP_C|GetMaxHealth _player))))