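; A destructible crate that breaks when hit by an actor tagged as a player projectile and can drop a health or ammo pickup.
; The first such hit applies damage and an impulse along the projectile's forward vector, then disables collision after a short delay.
; It spawns the item chosen by DroppedItem, then a timeline shrinks the shards from their saved scale before the actor destroys itself.
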(event OnComponentHit(Destructible)
  (params (HitComponent :type Primitive%20Component%20Object%20Reference) (OtherActor :type Actor%20Object%20Reference) (OtherComp :type Primitive%20Component%20Object%20Reference) (NormalImpulse :type Vector :default "0, 0, 0") (Hit :type Hit%20Result%20Structure%20%28by%20ref%29))
  (bind _destructible (Variables|Default|GetDestructible))
  ;[1 1 1] Crumble on projectile hit
  (if (not (Variables|Default|GetDestroyed))
    (if (Actor|ActorHasTag OtherActor "PlayerProjectile")
      (Class|DestructibleComponent|ApplyDamage _destructible 1e+02 (Transformation|GetWorldLocation _destructible) (Transformation|GetActorForwardVector OtherActor) (Variables|Default|GetImpulseStrength))
      (Variables|Default|SetDestroyed true)
      ;[1 1 1] Disable collision
      (Utilities|FlowControl|Delay 0.1)
      (Collision|SetCollisionEnabled (Variables|Default|GetDestructible) "NoCollision")
      ;[1 1 1] Spawn item
      (if (== (Variables|Default|GetDroppedItem) 1)
        (Game|SpawnActorfromClass "/Game/Pickups/BP_Health.BP_Health_C" (Math|Conversions|ToTransform(Vector) (Transformation|GetWorldLocation (Variables|Default|GetDestructible))) "AlwaysSpawn" 0 0)
        ;[1 1 1] Shrink pieces
        (bind _shardscale (Timeline|ShardShrink Play)
          (:Update
            (Transformation|SetRelativeScale3D (Variables|Default|GetDestructible) (* (Variables|Default|GetOriginalScale) _shardscale)))
          (:Finished
            (Actor|DestroyActor)))
        (elif (== (Variables|Default|GetDroppedItem) 2)
          (Game|SpawnActorfromClass "/Game/Pickups/BP_Ammo.BP_Ammo_C" (Math|Conversions|ToTransform(Vector) (Transformation|GetWorldLocation (Variables|Default|GetDestructible))) "AlwaysSpawn" 0 0)
          (Timeline|ShardShrink Play)
          (else
            (Timeline|ShardShrink Play)))))))

(event EventBeginPlay
  ;[1 1 1] Save scale of object (for destruction)
  (Variables|Default|SetOriginalScale (Transformation|GetWorldScale (Variables|Default|GetDestructible))))

(event Collision|EventActorBeginOverlap
  (params (OtherActor :type Actor%20Object%20Reference)))

(fn ConstructionScript)