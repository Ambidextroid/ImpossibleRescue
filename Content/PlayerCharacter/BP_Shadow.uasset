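; BP_Shadow is the player's shadow companion, which trails the player and moves to buttons to hack doors open.
; A looping timeline eases it toward a target by a fixed fraction each update, copying the target's rotation, while following is toggled on.
; The target is the player's ShadowLocation, or the button passed to DoorOpen, which plays a hacking sound and holds that state for the door opening time.
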(event EventBeginPlay
  (bind _asbp_player (Utilities|Casting|CastToBP_Player (Game|Player|GetPlayerPawn 0)))
  (Variables|Default|SetPlayerReference _asbp_player)
  ;[1 1 1] Following player
  (Timeline|Looping Play
    (:NewTrack_0
      (if (Variables|Default|GetFollowing)
        (if (Variables|Default|GetOpeningDoor)
          (CallFunction|NewFunction0 (Variables|Default|GetButton) 0.1)
          (else
            ;;[1 1 1] Follow player if not opening door
            (CallFunction|NewFunction0 (Variables|/Game/Blueprints/Pawns/BP_Player.BP_Player_C|GetShadowLocation (Variables|Default|GetPlayerReference)) 0.1)))))))

(event EventDoorOpen
  (params (Button :type Scene%20Component%20Object%20Reference))
  (Variables|Default|SetButton Button)
  (Variables|Default|SetOpeningDoor true)
  (Audio|PlaySoundatLocation (Variables|Default|GetDoorHackingSound) (Transformation|GetActorLocation) "0, 0, 0" 1.0 1.0 0.0 0 0 0)
  (Utilities|FlowControl|Delay (Variables|Default|GetDoorOpeningTime))
  (Utilities|FlowControl|Delay 0.1)
  (Variables|Default|SetOpeningDoor false))

(event EventShadowFollowToggle
  ;[1 1 1] Toggle follow behaviour
  (if (Variables|Default|GetFollowing)
    (Variables|Default|SetFollowing false)
    (else
      (Variables|Default|SetFollowing true))))

(fn ConstructionScript)

(fn NewFunction0
  (params (TargetLocationActor :type Scene%20Component%20Object%20Reference) (RateParameter :type Float%20%28single-precision%29))
  (bind _returnvalue (Transformation|GetWorldTransform TargetLocationActor))
  (bind _defaultsceneroot (Variables|Default|GetDefaultSceneRoot))
  (bind _returnvalue_2 (Transformation|GetWorldTransform _defaultsceneroot))
  (Transformation|SetWorldTransform (Variables|Default|GetDefaultSceneRoot) (Math|Transform|MakeTransform (+ (.location _returnvalue_2) (* (- (.location _returnvalue) (.location _returnvalue_2)) RateParameter)) (.rotation _returnvalue) (Transformation|GetWorldScale (Variables|Default|GetDefaultSceneRoot))) false false))