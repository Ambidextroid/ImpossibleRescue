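; Player character for a top-down shooter, with diagonal-axis movement, aiming, a shielded dash and a spawned shadow drone companion.
; Two spawned weapons share ammo and a heat pool, with a retriggerable delay and timeline driving cooldown and overheat lockout.
; Dispatchers report health, ammo and heat changes, and death shows the game-over menu.
; An overlap sphere sets the interact target and prompt, with interaction allowed only while the drone follows.
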(event OnComponentBeginOverlap(InteractSphere)
  (params (OverlappedComponent :type Primitive%20Component%20Object%20Reference) (OtherActor :type Actor%20Object%20Reference) (OtherComp :type Primitive%20Component%20Object%20Reference) (OtherBodyIndex :type Integer) (bFromSweep :type Boolean) (SweepResult :type Hit%20Result%20Structure%20%28by%20ref%29))
  ;[1 1 1] Interaction
  (UserInterface|Viewport|AddtoViewport (Variables|UI|GetInteractPrompt) 0)
  (Variables|Default|SetInteractable OtherActor))

(event OnComponentEndOverlap(InteractSphere)
  (params (OverlappedComponent :type Primitive%20Component%20Object%20Reference) (OtherActor :type Actor%20Object%20Reference) (OtherComp :type Primitive%20Component%20Object%20Reference) (OtherBodyIndex :type Integer))
  ;[1 1 1] Interaction
  (Widget|RemovefromParent (Variables|UI|GetInteractPrompt))
  (Variables|Default|SetInteractable 0))

(event Custom|HealthPickup
  (params (AddedHealth :type Float%20%28single-precision%29))
  (bind _maxhealth (Variables|Health|GetMaxHealth))
  ;[0.4235 1 0.5915] Health and Damage
  ;;[0.9826 1 0.8673] Add health
  (if (Variables|PlayerState|GetHealthCanChange)
    (bind _output_get (Variables|Health|SetHealth (Math|Float|Clamp(Float) (+ (Variables|Health|GetHealth) AddedHealth) 0.0 _maxhealth)))
    (Default|CallPlayerHealthUpdated (/ _output_get _maxhealth))))

(event Custom|AmmoPickup
  (params (AddedAmmo :type Integer))
  ;[1 0.07396 0.07396] Shooting
  ;;[1 1 1] Add ammo
  (bind _output_get (Variables|Shooting|SetAmmo (+ AddedAmmo (Variables|Shooting|GetAmmo))))
  (Default|CallPlayerAmmoUpdated _output_get))

(event Custom|DashEnded
  ;[1 0.9084 0.21] Movement
  ;;[1 1 1] Dashing
  (Dashing|EndDash)
  (Variables|PlayerState|SetShielded false)
  (Utilities|FlowControl|Delay (Variables|Dashing|GetDashCoolDown))
  (Variables|Dashing|SetDashRecovered true))

(event Custom|OnWeaponFired
  (params (Weapon :type BP%20Base%20Weapon%20Object%20Reference) (AmmoCost :type Integer))
  ;[1 0.07396 0.07396] Shooting
  ;;[1 1 1] Fire Weapon
  (if (and (>= (- (Variables|Shooting|GetAmmo) AmmoCost) 0) (not (Variables|Shooting|GetOverheated)))
    (Default|OnTriggerPull Weapon)
    (bind _output_get (Variables|Shooting|SetAmmo (- (Variables|Shooting|GetAmmo) AmmoCost)))
    (Default|CallPlayerAmmoUpdated _output_get)
    (Shooting|AddHeat AmmoCost)))

(event Custom|OnFiringStopped
  (params (Weapon :type BP%20Base%20Weapon%20Object%20Reference))
  ;[1 0.07396 0.07396] Shooting
  ;;[1 1 1] Stop Firing
  (Default|OnTriggerRelease Weapon))

(event Custom|HeatAdded
  ;[1 0.07396 0.07396] Shooting
  ;;[1 1 1] Control heat cooldown process
  (Utilities|FlowControl|RetriggerableDelay (Math|Float|SelectFloat (Variables|Default|GetOverheatCooldownDelay) (Variables|Default|GetStandardCooldownDelay) (Variables|Shooting|GetOverheated)))
  (Timeline|Cooldown PlayFromStart
    (:Update
      (Shooting|ReduceHeat))))

(event Custom|CooldownComplete
  ;[1 0.07396 0.07396] Shooting
  ;;[1 1 1] Control heat cooldown process
  (Timeline|Cooldown Stop
    (:Update
      (Shooting|ReduceHeat))))

(event Custom|AimDirectionEvent
  (params (Direction :type Vector))
  (bind _returnvalue (Game|GetPlayerController 0))
  (bind _weapon1spawn (Variables|Default|GetWeapon1Spawn))
  (bind _hitresult (Game|Player|GetHitResultUnderCursorbyChannel _returnvalue "TraceTypeQuery3" true))
  (bind _returnvalue_2 (Transformation|GetWorldLocation _weapon1spawn))
  (bind _returnvalue_3 (Math|Vector|GetUnitDirection(Vector) _returnvalue_2 (.location _hitresult)))
  ;[1 0.9084 0.21] Movement
  ;;[1 1 1] Rotate
  (if (Variables|PlayerState|GetCanMove)
    (Transformation|SetWorldRotation (Variables|Collision|GetCapsuleComponent) (Math|Conversions|RotationFromXVector (Math|Vector|MakeVector (.x Direction) (.y Direction) 0.0)) false false)
    (if (<= (Class|KismetMathLibrary|DegAcos (Math|Vector|DotProduct (Math|Vector|Normalize (Math|Vector|MakeVector (.x Direction) (.y Direction) 0.0)) (Math|Vector|Normalize (Math|Vector|MakeVector (.x _returnvalue_3) (.y _returnvalue_3) 0.0)))) 2e+01)
      (Transformation|SetWorldRotation _weapon1spawn (Math|Conversions|RotationFromXVector (Math|Vector|MakeVector (.x _returnvalue_3) (.y _returnvalue_3) 0.0)) false false))))

(event EventBeginPlay
  (bind _weapon1spawn (Variables|Default|GetWeapon1Spawn))
  (bind _weapon2spawn (Variables|Default|GetWeapon2Spawn))
  (bind _charactermovement (Variables|Character|GetCharacterMovement))
  (bind _returnvalue (Transformation|GetWorldTransform _weapon2spawn))
  (bind _returnvalue_2 (Transformation|GetWorldTransform _weapon1spawn))
  ;[0 0.8904 1] Initial Setup
  (Utilities|FlowControl|Sequence
    (:then_0
      ;;[1 1 1] Spawn shadow drone
      (bind _returnvalue_3 (Game|SpawnActorfromClass "/Game/PlayerCharacter/BP_Shadow.BP_Shadow_C" (Math|Transform|MakeTransform (Transformation|GetWorldLocation (Variables|Collision|GetCapsuleComponent)) "0, 0, 0" "1,1,1") "Undefined" 0 0))
      (Variables|Default|SetShadowReference _returnvalue_3))
    (:then_1
      ;;[1 1 1] Spawn SMG
      (bind _returnvalue_4 (Game|SpawnActorfromClass "/Game/PlayerCharacter/Weapons/BP_Pistol.BP_Pistol_C" (Math|Transform|MakeTransform (.location _returnvalue_2) (.rotation _returnvalue_2) "1,1,1") "AlwaysSpawn" 0 0))
      (bind _output_get (Variables|Shooting|SetWeapon1 _returnvalue_4))
      (Transformation|AttachComponentToComponent _output_get (Variables|Default|GetWeapon1Spawn) "None" "SnapToTarget" "SnapToTarget" "KeepRelative" true))
    (:then_2
      ;;[1 1 1] Spawn Shotgun
      (bind _returnvalue_5 (Game|SpawnActorfromClass "/Game/PlayerCharacter/Weapons/BP_Shotgun.BP_Shotgun_C" (Math|Transform|MakeTransform (.location _returnvalue) (.rotation _returnvalue) "1,1,1") "AlwaysSpawn" 0 0))
      (bind _output_get_2 (Variables|Shooting|SetWeapon2 _returnvalue_5))
      (Transformation|AttachComponentToComponent _output_get_2 (Variables|Default|GetWeapon2Spawn) "None" "SnapToTarget" "SnapToTarget" "KeepRelative" true))
    (:then_3
      ;;[1 1 1] Set Up HUD
      (bind _returnvalue_6 (UserInterface|CreateWidget "/Game/UI/Widgets/WBP_PlayerHUD.WBP_PlayerHUD_C" 0 self))
      (UserInterface|Viewport|AddtoViewport _returnvalue_6 0)
      (Default|CallPlayerHealthUpdated (/ (Variables|Health|GetHealth) (Variables|Health|GetMaxHealth)))
      (Default|CallPlayerAmmoUpdated (Variables|Shooting|GetAmmo))
      (bind _returnvalue_7 (UserInterface|CreateWidget "/Game/UI/Widgets/WBP_InteractPrompt.WBP_InteractPrompt_C"))
      (Variables|UI|SetInteractPrompt _returnvalue_7))
    (:then_4
      ;;[1 1 1] Set up dash
      ;;;[1 1 1] Note default speed
      (Variables|Dashing|SetDefaultSpeed (Variables|/Script/Engine.CharacterMovementComponent|GetMaxWalkSpeed _charactermovement))
      (Variables|Dashing|SetDefaultAcceleration (Class|CharacterMovementComponent|GetMaxAcceleration _charactermovement))
      (Variables|Dashing|SetDashSpeed (/ (Variables|Dashing|GetDashDistance) (Variables|Dashing|GetDashDuration))))))

(event Game|Damage|EventAnyDamage
  (params (Damage :type Float%20%28single-precision%29) (DamageType :type Damage%20Type%20Object%20Reference) (InstigatedBy :type Controller%20Object%20Reference) (DamageCauser :type Actor%20Object%20Reference))
  ;[0.4235 1 0.5915] Health and Damage
  ;;[1 1 1] Player damage
  (if (and (not (Variables|PlayerState|GetShielded)) (Variables|PlayerState|GetHealthCanChange))
    (bind _output_get (Variables|Health|SetHealth (- (Variables|Health|GetHealth) Damage)))
    (Default|CallPlayerHealthUpdated (/ _output_get (Variables|Health|GetMaxHealth)))
    (if (<= _output_get 0.0)
      (Health|Die))))

(event Input|ActionEvents|InputActionEscape
  (params (Key :type Key%20Structure :default "None"))
  ;[1 1 1] Temporary Way to quit from standalone
  (:Pressed
    (Game|QuitGame 0 "Quit" false)))

(event Input|ActionEvents|InputActionWeapon1
  (params (Key :type Key%20Structure :default "None"))
  (bind _weapon1 (Variables|Shooting|GetWeapon1))
  ;[1 0.07396 0.07396] Shooting
  ;;[1 1 1] Fire Weapons
  (:Pressed
    (CallFunction|OnWeaponFired _weapon1 (Variables|Shooting|GetSMGAmmoCost)))
  (:Released
    (CallFunction|OnFiringStopped _weapon1)))

(event Input|ActionEvents|InputActionInteract
  (params (Key :type Key%20Structure :default "None"))
  (bind _interactable (Variables|Default|GetInteractable))
  ;[1 1 1] Interactions
  (:Pressed
    (if (Variables|/Game/PlayerCharacter/BP_Shadow.BP_Shadow_C|GetFollowing (Variables|Default|GetShadowReference))
      (Default|CallDoorInteractDispatcher)
      (if (Utilities|IsValid _interactable)
        (Class|IInteractable|Interacted(Message) _interactable)))))

(event Input|ActionEvents|InputActionDash
  (params (Key :type Key%20Structure :default "None"))
  ;[1 0.9084 0.21] Movement
  ;;[1 1 1] Dashing
  (:Pressed
    (if (and (Variables|Dashing|GetDashRecovered) (Variables|PlayerState|GetCanMove))
      (Variables|Dashing|SetDashRecovered false)
      (Variables|PlayerState|SetShielded true)
      (Dashing|StartDash)
      (Utilities|Time|SetTimerbyEvent (delegate Custom|DashEnded) (Variables|Dashing|GetDashDuration)))))

(event Input|ActionEvents|InputActionWeapon2
  (params (Key :type Key%20Structure :default "None"))
  (bind _weapon2 (Variables|Shooting|GetWeapon2))
  ;[1 0.07396 0.07396] Shooting
  ;;[1 1 1] Fire Weapons
  (:Pressed
    (CallFunction|OnWeaponFired _weapon2 (Variables|Shooting|GetShotgunAmmoCost)))
  (:Released
    (CallFunction|OnFiringStopped _weapon2)))

(event Input|AxisEvents|InputAxisMoveForward
  (params (AxisValue :type Float%20%28single-precision%29))
  ;[1 0.9084 0.21] Movement
  ;;[1 1 1] Arrow key movement
  (Pawn|Input|AddMovementInput "1.000000,-1.000000, 0" AxisValue false))

(event Input|AxisEvents|InputAxisMoveRight
  (params (AxisValue :type Float%20%28single-precision%29))
  ;[1 0.9084 0.21] Movement
  ;;[1 1 1] Arrow key movement
  (Pawn|Input|AddMovementInput "1.000000,1.000000, 0" AxisValue false))

(event Input|KeyboardEvents|Q
  (params (Key :type Key%20Structure :default "None"))
  ;[0.05104 0.05104 0.05104] Shadow Logic
  ;;[1 1 1] Toggle Shadow Follow
  (:Pressed
    (Class|BPIShadow|ShadowFollowToggle(Message) (Variables|Default|GetShadowReference))))

(fn ConstructionScript)

(fn Die
  (Input|DisableInput 0)
  (Rendering|SetVisibility (Variables|Character|GetMesh) false false)
  (bind _returnvalue (UserInterface|CreateWidget "/Game/UI/Widgets/WBP_GameOverMenu.WBP_GameOverMenu_C"))
  (UserInterface|Viewport|AddtoViewport _returnvalue 0)
  (Variables|PlayerState|SetCanMove false)
  (Variables|PlayerState|SetHealthCanChange false))

(fn EndDash
  (bind _charactermovement (Variables|Character|GetCharacterMovement))
  (Variables|/Script/Engine.CharacterMovementComponent|SetMaxWalkSpeed _charactermovement (Variables|Dashing|GetDefaultSpeed))
  (Variables|/Script/Engine.CharacterMovementComponent|SetMaxAcceleration _charactermovement (Variables|Dashing|GetDefaultAcceleration)))

(fn StartDash
  (bind _charactermovement (Variables|Character|GetCharacterMovement))
  (Variables|/Script/Engine.CharacterMovementComponent|SetMaxWalkSpeed _charactermovement (Variables|Dashing|GetDashSpeed))
  (Variables|/Script/Engine.CharacterMovementComponent|SetMaxAcceleration _charactermovement (Variables|Dashing|GetMax%20Acceleration)))

(fn AddHeat
  (params (AmmoCount :type Integer))
  (bind _maxheat (Variables|Shooting|GetMaxHeat))
  (Variables|Shooting|SetOverheated (>= (+ (Variables|Shooting|GetHeat) (* (Variables|Shooting|GetHeatPerShot) (Math|Conversions|ToFloat(Integer) AmmoCount))) _maxheat))
  (bind _output_get (Variables|Shooting|SetHeat (Math|Float|Min(Float) (+ (Variables|Shooting|GetHeat) (* (Variables|Shooting|GetHeatPerShot) (Math|Conversions|ToFloat(Integer) AmmoCount))) _maxheat)))
  (Default|CallWeaponHeatUpdated _output_get (Variables|Shooting|GetOverheated))
  (CallFunction|HeatAdded))

(fn ReduceHeat
  (bind _output_get (LocalVariables|SetBelowZero (< (- (Variables|Shooting|GetHeat) (* (Variables|Shooting|GetCooldownRate) (Utilities|Time|GetWorldDeltaSeconds))) 0.0)))
  ;[1 1 1] Can only still be overheated if was overheated on last frame and heat still above 0
  (Variables|Shooting|SetOverheated (and (Variables|Shooting|GetOverheated) (not _output_get)))
  (bind _output_get_2 (Variables|Shooting|SetHeat (Math|Float|Max(Float) (- (Variables|Shooting|GetHeat) (* (Variables|Shooting|GetCooldownRate) (Utilities|Time|GetWorldDeltaSeconds))) 0.0)))
  (Default|CallWeaponHeatUpdated _output_get_2 (Variables|Shooting|GetOverheated))
  (if (LocalVariables|GetBelowZero)
    (CallFunction|CooldownComplete)))