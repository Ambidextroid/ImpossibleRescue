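; Player shotgun weapon that damages every enemy inside a cone-shaped hit area when the trigger is pulled.
; With ammo available, each shot spawns a Niagara effect at the emitter point, spends one round and gathers enemies overlapping HitCone.
; A visibility trace toward each enemy supplies a hit distance for linear damage falloff, without checking whether that enemy is the actor hit.
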(event EventBeginPlay
  (|CallParentFunction) ; This node is disabled and will not be called.\nDrag off pins to build functionality.
)

(event Collision|EventActorBeginOverlap
  (params (OtherActor :type Actor%20Object%20Reference))
  (|CallParentFunction OtherActor) ; This node is disabled and will not be called.\nDrag off pins to build functionality.
)

(event EventTick
  (params (DeltaSeconds :type Float%20%28single-precision%29))
  (|CallParentFunction DeltaSeconds) ; This node is disabled and will not be called.\nDrag off pins to build functionality.
)

(event EventOnTriggerPull
  (bind _emitterpoint (Variables|Default|GetEmitterPoint))
  (bind _returnvalue (Transformation|GetWorldTransform _emitterpoint))
  ;[1 1 1] Damage enemies
  (if (> (Variables|Default|GetAmmo) 0)
    (Niagara|SpawnSystematLocation "/Game/PlayerCharacter/Weapons/NS_Shotgun.NS_Shotgun" (.location _returnvalue) (.rotation _returnvalue))
    (Math|Integer|DecrementInt (Variables|Default|GetAmmo)
      (:%20%20
        (for _array_element (Collision|GetOverlappingActors (Variables|Default|GetHitCone) "/Game/Enemies/BP_EnemyBase.BP_EnemyBase_C" :!class /Script/Engine.PrimitiveComponent)
          (bind _outhit (Collision|LineTraceByChannel (Transformation|GetWorldLocation (Variables|Default|GetArrow)) (Transformation|GetActorLocation _array_element) "TraceTypeQuery1" false 0 "None"))
          (Game|Damage|ApplyDamage _array_element (|((((NegativeOne*x)+dist)/dist)*dmg) (.distance _outhit) 6e+02 1e+02 -1.0) 0 0))))))

(fn ConstructionScript
  (|CallParentFunction))