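; Deprecated ACT2 patrol enemy Blueprint that defines left/right movement along the world X axis.
; Movement flips direction by IsMovingLeft and applies forced movement input scaled by MoveSpeed and frame delta time, or calls CountMovementPaused while paused.
; Event graph nodes are disabled placeholders, and nothing in this file calls Movement or changes direction.
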(event EventBeginPlay
  (|CallParentFunction) ; This node is disabled and will not be called.\nDrag off pins to build functionality.
)

(event Collision|EventActorBeginOverlap
  (params (OtherActor :type Actor%20Object%20Reference))
  (|CallParentFunction OtherActor) ; This node is disabled and will not be called.\nDrag off pins to build functionality.
)

(event EventTick
  (params (DeltaSeconds :type Float%20%28single-precision%29))
  (|CallParentFunction DeltaSeconds) ; This node is disabled and will not be called.\nDrag off pins to build functionality.
)

(fn ConstructionScript
  (|CallParentFunction))

(fn Movement
  (if (Variables|Default|GetIsMovementPaused)
    (CallFunction|CountMovementPaused)
    (else
      (if (Variables|Default|GetIsMovingLeft)
        (LocalVariables|SetMovementModifier -1.0)
        (else
          (LocalVariables|SetMovementModifier 1.0)))
      (Pawn|Input|AddMovementInput (Math|Vector|MakeVector (* (LocalVariables|GetMovementModifier) (Variables|Default|GetMoveSpeed) (Utilities|Time|GetWorldDeltaSeconds)) 0.0 0.0) 1.0 true))))