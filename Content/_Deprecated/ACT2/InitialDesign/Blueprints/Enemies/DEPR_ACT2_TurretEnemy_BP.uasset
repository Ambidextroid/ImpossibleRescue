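; Deprecated ACT2 turret enemy Blueprint that replaces its parent's shot with a timed burst of bullets.
; Shoot calls BurstFire, which clears CanFire and starts a looping timer that runs FireBurstShot to fire a bullet and count it.
; TrackFireStatus extends the parent version with TrackBurstFire, which clears the timer and resets the count once the burst limit is reached.
; The event graph holds only disabled placeholder events.
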(event EventBeginPlay
  (|CallParentFunction) ; This node is disabled and will not be called.\nDrag off pins to build functionality.
)

(event Collision|EventActorBeginOverlap
  (params (OtherActor :type Actor%20Object%20Reference))
  (|CallParentFunction OtherActor) ; This node is disabled and will not be called.\nDrag off pins to build functionality.
)

(event EventTick
  (params (DeltaSeconds :type Float%20%28single-precision%29))
  (|CallParentFunction DeltaSeconds) ; This node is disabled and will not be called.\nDrag off pins to build functionality.
)

(fn ConstructionScript
  (|CallParentFunction))

(fn BurstFire
  (Variables|Default|SetCanFire false)
  (bind _returnvalue (Utilities|Time|SetTimerbyFunctionName 0 "FireBurstShot" (Variables|Default|GetBurstFireDelay) true))
  (Variables|Default|SetBurstFireTimerHandle _returnvalue))

(fn Shoot
  (CallFunction|BurstFire))

(fn FireBurstShot
  (CallFunction|FireBullet)
  (Variables|Default|SetBurstShotsFired (+ (Variables|Default|GetBurstShotsFired) 1)))

(fn TrackBurstFire
  (if (>= (Variables|Default|GetBurstShotsFired) (Variables|Default|GetBurstShotsMax))
    (Utilities|Time|ClearandInvalidateTimerbyHandle (Variables|Default|GetBurstFireTimerHandle))
    (Variables|Default|SetBurstShotsFired 0)))

(fn TrackFireStatus
  (|CallParentFunction)
  (CallFunction|TrackBurstFire))