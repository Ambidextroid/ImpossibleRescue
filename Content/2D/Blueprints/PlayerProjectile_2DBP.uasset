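; Projectile Blueprint for the 2D game, representing shots that belong to the player.
; CheckForTarget ignores any collision class derived from Player_2DBP; for anything else it sends ProjectileCollisionMessage to the target and destroys the projectile.
; The event graph holds only disabled default events and the construction script just calls its parent, so this file does not show movement or what triggers the check.
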(event EventBeginPlay
  (|CallParentFunction) ; This node is disabled and will not be called.\nDrag off pins to build functionality.
)

(event Collision|EventActorBeginOverlap
  (params (OtherActor :type Actor%20Object%20Reference))
  (|CallParentFunction OtherActor) ; This node is disabled and will not be called.\nDrag off pins to build functionality.
)

(event EventTick
  (params (DeltaSeconds :type Float%20%28single-precision%29))
  (|CallParentFunction DeltaSeconds) ; This node is disabled and will not be called.\nDrag off pins to build functionality.
)

(fn ConstructionScript
  (|CallParentFunction))

(fn CheckforTarget
  (params (Collision%20Target :type Actor%20Object%20Reference) (Collision%20Class :type Actor%20Class%20Reference))
  (if (not (Utilities|ClassIsChildOf Collision%20Class "/Game/2D/Blueprints/Player_2DBP.Player_2DBP_C"))
    (Class|DamageInterface2DInterface|ProjectileCollision(Message) Collision%20Target)
    (Actor|DestroyActor)))