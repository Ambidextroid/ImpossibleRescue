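; A 2D pickup actor that flies to the player and destroys itself when the player overlaps its Box trigger.
; Once triggered, Tick calls MoveToPlayer, which grows an alpha by speed times delta time and lerps from the spawn location toward the player's current position.
; It destroys itself within a finish range of the player; no reward or effect is applied here.
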(event OnComponentBeginOverlap(Box)
  (params (OverlappedComponent :type Primitive%20Component%20Object%20Reference) (OtherActor :type Actor%20Object%20Reference) (OtherComp :type Primitive%20Component%20Object%20Reference) (OtherBodyIndex :type Integer) (bFromSweep :type Boolean) (SweepResult :type Hit%20Result%20Structure%20%28by%20ref%29))
  (if (== OtherActor (Variables|Default|GetPlayer))
    (Variables|Default|SetIsMovingToPlayer true)))

(event EventBeginPlay
  (Variables|Default|SetPlayer (Game|Player|GetPlayerPawn 0))
  (Variables|Default|SetStartPos (Transformation|GetActorLocation)))

(event Collision|EventActorBeginOverlap
  (params (OtherActor :type Actor%20Object%20Reference)))

(event EventTick
  (params (DeltaSeconds :type Float%20%28single-precision%29))
  (if (Variables|Default|GetIsMovingToPlayer)
    (CallFunction|MovetoPlayer)))

(fn ConstructionScript)

(fn MovetoPlayer
  (bind _player (Variables|Default|GetPlayer))
  (bind _returnvalue (Transformation|GetActorLocation _player))
  ;[1 1 1] Update Interpolation
  (Variables|Default|SetInterpolation (+ (* (Variables|Default|GetInterpolationSpeed) (Utilities|Time|GetWorldDeltaSeconds)) (Variables|Default|GetInterpolation)))
  (Transformation|SetActorLocation (Math|Vector|Lerp(Vector) (Variables|Default|GetStartPos) _returnvalue (Variables|Default|GetInterpolation)) false false)
  (if (<= (Math|Vector|Distance(Vector) (Math|Vector|Lerp(Vector) (Variables|Default|GetStartPos) _returnvalue (Variables|Default|GetInterpolation)) _returnvalue) (Variables|Default|GetRangeToFinishPickup))
    (Actor|DestroyActor)))