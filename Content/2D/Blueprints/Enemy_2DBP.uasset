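; Base 2D enemy Blueprint that shoots at the player when within attack range and explodes when hit by a projectile.
; Each tick it updates a fire-rate timer, calls Movement if enabled, checks distance to player pawn 0 and fires when ready.
; Shots spawn an enemy projectile on the enemy's X/Z position, aimed at the player's current location.
; Movement is an empty function, and a projectile collision spawns an explosion and destroys the actor.
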(event EventBeginPlay
  (Variables|Default|SetPlayer (Game|Player|GetPlayerPawn 0)))

(event Collision|EventActorBeginOverlap
  (params (OtherActor :type Actor%20Object%20Reference)))

(event EventTick
  (params (DeltaSeconds :type Float%20%28single-precision%29))
  (CallFunction|TrackFireStatus)
  (if (Variables|Default|GetHasMovement)
    (CallFunction|Movement))
  (CallFunction|DistanceCheck)
  (if (Variables|Default|GetCanFire)
    (if (Variables|Default|GetPlayerIsInRange)
      (CallFunction|Shoot))))

(event EventProjectileCollision
  (CallFunction|Destroy))

(fn ConstructionScript)

(fn DistanceCheck
  (Variables|Default|SetPlayerIsInRange (<= (Math|Vector|Distance(Vector) (Transformation|GetActorLocation) (Transformation|GetActorLocation (Variables|Default|GetPlayer))) (Variables|Default|GetAttackDist))))

(fn Shoot
  (bind _returnvalue (Transformation|GetActorLocation))
  (bind _returnvalue_2 (Game|SpawnActorfromClass "/Game/2D/Blueprints/EnemyProjectile_2DBP.EnemyProjectile_2DBP_C" (Math|Transform|MakeTransform (Math|Vector|MakeVector (.x _returnvalue) 0.0 (.z _returnvalue)) "0, 0, 0" "1,1,1") "Undefined" 0 0))
  (Default|SetDir _returnvalue_2 (Math|Vector|GetUnitDirection(Vector) (Transformation|GetActorLocation) (Transformation|GetActorLocation (Variables|Default|GetPlayer))))
  (Variables|Default|SetCanFire false))

(fn Movement)

(fn Destroy
  (Game|SpawnActorfromClass "/Game/2D/Blueprints/Explosion_2DBP.Explosion_2DBP_C" (Math|Transform|MakeTransform (Transformation|GetActorLocation) "0, 0, 0" "1,1,1") "Undefined" 0 0)
  (Actor|DestroyActor))

(fn TrackFireStatus
  (if (not (Variables|Default|GetCanFire))
    (bind _output_get (Variables|Default|SetTimeSinceLastFire (+ (Variables|Default|GetTimeSinceLastFire) (Utilities|Time|GetWorldDeltaSeconds))))
    (if (>= _output_get (Variables|Default|GetFireRate))
      (Variables|Default|SetCanFire true)
      (Variables|Default|SetTimeSinceLastFire 0.0))))