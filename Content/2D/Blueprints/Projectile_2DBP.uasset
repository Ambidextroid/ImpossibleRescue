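; Base-level 2D projectile actor that flies in a set direction and destroys itself on any overlap or when its lifetime expires.
; Tick moves it by direction and speed without sweeping, then accumulates lifetime.
; SetDir stores the direction and sets pitch from a look-at rotation, adjusted for negative X, printing the angle.
; SetDamage stores a value, but overlaps neither apply damage nor filter targets.
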(event EventBeginPlay)

(event Collision|EventActorBeginOverlap
  (params (OtherActor :type Actor%20Object%20Reference))
  (CallFunction|CheckforTarget OtherActor (Utilities|GetClass OtherActor)))

(event EventTick
  (params (DeltaSeconds :type Float%20%28single-precision%29))
  (CallFunction|Move)
  (CallFunction|LifetimeCheck))

(fn ConstructionScript)

(fn Move
  (Transformation|SetActorLocation (+ (Transformation|GetActorLocation) (* (Variables|Default|GetMoveDir) (* (Variables|Default|GetSpeed) (Utilities|Time|GetWorldDeltaSeconds)))) false false))

(fn SetDir
  (params (Direction :type Vector))
  (bind _returnvalue (Transformation|GetActorLocation))
  (bind _output_get (Variables|Default|SetMoveDir (* Direction 1.0)))
  (bind _angle_out (CallFunction|AngleOffset (.pitch (Math|Rotator|FindLookatRotation _returnvalue (+ _returnvalue _output_get)))))
  (Transformation|SetActorRotation (Math|Rotator|MakeRotator 0.0 _angle_out 0.0))
  (Development|PrintString (Utilities|String|ToString(Float) _angle_out)))

(fn LifetimeCheck
  (bind _output_get (Variables|Default|SetCurrentLifetime (+ (Variables|Default|GetCurrentLifetime) (Utilities|Time|GetWorldDeltaSeconds))))
  (if (>= _output_get (Variables|Default|GetMaxLifetime))
    (Actor|DestroyActor)))

(fn AngleOffset
  (params (Angle%20In :type Float%20%28single-precision%29))
  (if (>= (.x (Variables|Default|GetMoveDir)) 0.0)
    (return Angle%20In)
    (else
      (return (- 3.6e+02 Angle%20In)))))

(fn CheckforTarget
  (params (Collision%20Target :type Actor%20Object%20Reference) (Collision%20Class :type Actor%20Class%20Reference))
  (Actor|DestroyActor))

(fn SetDamage
  (params (Damage :type Float%20%28single-precision%29))
  (Variables|Default|SetDamage Damage))