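; 2D health pickup Blueprint that restores health to the player when collected.
; It overrides CanPickup to allow collection only while the player's Health is below MaxHealth.
; OnPickup passes its HealthValue to the player through HealthPickupMessage, leaving the actual healing to the player.
; The event graph and construction script add no logic of their own.
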(event EventBeginPlay
  (|CallParentFunction) ; This node is disabled and will not be called.\nDrag off pins to build functionality.
)

(event EventTick
  (params (DeltaSeconds :type Float%20%28single-precision%29))
  (|CallParentFunction DeltaSeconds) ; This node is disabled and will not be called.\nDrag off pins to build functionality.
)

(fn ConstructionScript
  (|CallParentFunction))

(fn OnPickup
  (Class|PickupInterface2DInterface|HealthPickup(Message) (Variables|Default|GetPlayer) (Variables|Default|GetHealthValue)))

(fn CanPickup
  (bind _player (Variables|Default|GetPlayer))
  (return (< (Variables|/Game/2D/Blueprints/Player/Player_2DBP.Player_2DBP_C|GetHealth _player) (Variables|/Game/2D/Blueprints/Player/Player_2DBP.Player_2DBP_C|GetMaxHealth _player))))