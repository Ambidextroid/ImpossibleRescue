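; 2D player character that moves along X, jumps and shoots projectiles toward the mouse cursor.
; Horizontal input offsets the actor's location directly without sweep, scaled by speed and frame time, and rotates the sprite to face the movement direction.
; Jump launches the character only when it is not falling.
; Firing spawns PlayerProjectile_2DBP and aims it in the XZ plane at the deprojected cursor position; ProjectileCollision only prints a hit message.
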(event EventBeginPlay
  (Variables|/Script/Engine.PlayerController|SetbShowMouseCursor (Game|GetPlayerController 0) true))

(event Collision|EventActorBeginOverlap
  (params (OtherActor :type Actor%20Object%20Reference)))

(event EventTick
  (params (DeltaSeconds :type Float%20%28single-precision%29)))

(event EventProjectileCollision
  (Development|PrintString "Player Hit"))

(event Input|ActionEvents|InputActionJump
  (params (Key :type Key%20Structure :default "None"))
  (:Pressed
    (if (not (AI|Components|NavMovement|IsFalling (Variables|Character|GetCharacterMovement)))
      (Character|LaunchCharacter (Math|Vector|MakeVector 0.0 0.0 (Variables|Default|GetJumpHeight)) false false))))

(event Input|ActionEvents|InputActionFire
  (params (Key :type Key%20Structure :default "None"))
  (:Pressed
    (CallFunction|ShootProjectile)))

(event Input|AxisEvents|InputAxisMoveHorizontal_2D
  (params (AxisValue :type Float%20%28single-precision%29))
  (CallFunction|Movement AxisValue))

(fn ConstructionScript)

(fn Movement
  (params (MoveValue :type Float%20%28single-precision%29))
  (bind _returnvalue (Utilities|Time|GetWorldDeltaSeconds))
  (bind _movespeed (Variables|Default|GetMoveSpeed))
  (bind _returnvalue_2 (* MoveValue _movespeed _returnvalue))
  ;[1 1 1] Calculating movement values
  ;[1 1 1] Checking whether the sprite should flip based on current movement input
  (if (> _returnvalue_2 0.0)
    (Variables|Default|SetIsMovingLeft false)
    (CallFunction|FlipSprite :!label _label)
    (Transformation|SetActorLocation (+ (Transformation|GetActorLocation) (Math|Vector|MakeVector _returnvalue_2 0.0 0.0)) false false)
    (elif (< _returnvalue_2 0.0)
      (Variables|Default|SetIsMovingLeft true)
      (goto _label))))

(fn FlipSprite
  (bind _sprite (Variables|Default|GetSprite))
  (if (Variables|Default|GetIsMovingLeft)
    (Transformation|SetRelativeRotation _sprite "0,180.000000, 0" false false)
    (else
      (Transformation|SetRelativeRotation _sprite "0, 0, 0" false false))))

(fn ShootProjectile
  (bind _returnvalue (Game|GetPlayerController 0))
  (bind _returnvalue_2 (Transformation|GetActorLocation))
  (bind _worldlocation (Game|Player|ConvertMouseLocationToWorldSpace _returnvalue))
  (bind _returnvalue_3 (Game|SpawnActorfromClass "/Game/2D/Blueprints/PlayerProjectile_2DBP.PlayerProjectile_2DBP_C" (Math|Transform|MakeTransform (Math|Vector|MakeVector (.x _returnvalue_2) 0.0 (.z _returnvalue_2)) "0, 0, 0" "1,1,1") "Undefined" 0 0))
  (Default|SetDir _returnvalue_3 (Math|Vector|GetUnitDirection(Vector) (Math|Vector|MakeVector (.x _returnvalue_2) 0.0 (.z _returnvalue_2)) (Math|Vector|MakeVector (.x _worldlocation) 0.0 (.z _worldlocation)))))