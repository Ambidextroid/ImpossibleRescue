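; BP_BackgroundSound is an audio actor that plays a set of background sound cues and follows the game's pause state.
; On BeginPlay it creates an audio component per cue, with a nested loop that replays all components so far and rebinds to BP_GameModeBase dispatchers after each addition.
; Game paused and level completed events pause every component, and game unpaused resumes them.
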(event Custom|PauseSounds
  (for _array_element (Variables|Default|GetAudioComponents)
    (Class|AudioComponent|SetPaused _array_element true)))

(event Custom|UnpauseSounds
  (for _array_element (Variables|Default|GetAudioComponents)
    (Class|AudioComponent|SetPaused _array_element false)))

(event EventBeginPlay
  (for _array_element (Variables|Default|GetSoundCues)
    (bind _returnvalue (AddComponent|AddAudioComponent false))
    (Utilities|Array|Add (Variables|Default|GetAudioComponents) _returnvalue)
    (Audio|Components|Audio|SetSound _returnvalue _array_element)
    (for _array_element_2 (Variables|Default|GetAudioComponents)
      (Audio|Components|Audio|Play _array_element_2 0.0)
      (bind _asbp_game_mode_base (Utilities|Casting|CastToBP_GameModeBase (Game|GetGameMode)))
      (EventDispatchers|BindEventtoGamePausedDispatcher _asbp_game_mode_base (delegate Custom|PauseSounds))
      (EventDispatchers|BindEventtoGameUnpausedDispatcher _asbp_game_mode_base (delegate Custom|UnpauseSounds))
      (EventDispatchers|BindEventtoLevelCompletedDispatcher _asbp_game_mode_base (delegate Custom|PauseSounds)))))

(event EventTick
  (params (DeltaSeconds :type Float%20%28single-precision%29)))

(fn ConstructionScript)