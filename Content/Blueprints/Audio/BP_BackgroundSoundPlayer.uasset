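; Background sound player actor that plays a set of sound cues and follows the game's pause state.
; On BeginPlay it creates an audio component per SoundCues entry at runtime, since an editable component array cannot be assigned cues directly.
; Nested loops play the stored components and bind to BP_GameModeBase dispatchers, repeating as each is added.
; Pause and level completion pause all components, and unpause resumes them.
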(event Custom|PauseSounds
  ;[1 1 1] Pause sounds
  (for _array_element (Variables|Default|GetAudioComponents)
    (Class|AudioComponent|SetPaused _array_element true)))

(event Custom|UnpauseSounds
  ;[1 1 1] Unpause sounds
  (for _array_element (Variables|Default|GetAudioComponents)
    (Class|AudioComponent|SetPaused _array_element false)))

(event EventBeginPlay
  ;[1 1 1] Set up audio components: if you just make the audio component array public editable, that's fine but it won't let you set the sound cues for the audio components to play: it'll want actual, existing audio components. There must be a nicer way of doing this
  (for _array_element (Variables|Default|GetSoundCues)
    (bind _returnvalue (AddComponent|AddAudioComponent false))
    (Utilities|Array|Add (Variables|Default|GetAudioComponents) _returnvalue)
    (Audio|Components|Audio|SetSound _returnvalue _array_element)
    ;[1 1 1] Play all background sounds
    (for _array_element_2 (Variables|Default|GetAudioComponents)
      (Audio|Components|Audio|Play _array_element_2 0.0)
      (bind _asbp_game_mode_base (Utilities|Casting|CastToBP_GameModeBase (Game|GetGameMode)))
      (EventDispatchers|BindEventtoGamePausedDispatcher _asbp_game_mode_base (delegate Custom|PauseSounds))
      (EventDispatchers|BindEventtoGameUnpausedDispatcher _asbp_game_mode_base (delegate Custom|UnpauseSounds))
      (EventDispatchers|BindEventtoLevelCompletedDispatcher _asbp_game_mode_base (delegate Custom|PauseSounds)))))

(fn ConstructionScript)