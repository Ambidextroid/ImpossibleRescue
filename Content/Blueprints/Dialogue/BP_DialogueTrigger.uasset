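; BP_DialogueTrigger is a one-shot trigger volume that starts a dialogue when the player walks into it.
; On BeginPlay it finds and caches the level's BP_DialogueManager, or logs an error and destroys itself if none exists.
; When a BP_Player overlaps the Box while no dialogue is active, it passes DialogueToTrigger to the manager and then destroys itself.
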(event OnComponentBeginOverlap(Box)
  (params (OverlappedComponent :type Primitive%20Component%20Object%20Reference) (OtherActor :type Actor%20Object%20Reference) (OtherComp :type Primitive%20Component%20Object%20Reference) (OtherBodyIndex :type Integer) (bFromSweep :type Boolean) (SweepResult :type Hit%20Result%20Structure%20%28by%20ref%29))
  (bind _dialoguemanager (Variables|Default|GetDialogueManager))
  ;[1 1 1] Check if the colliding actor is a player, and whether dialogue is already active
  (if (not (Variables|/Game/Blueprints/Dialogue/BP_DialogueManager.BP_DialogueManager_C|GetIsDialogueActive _dialoguemanager))
    (if (Utilities|ClassIsChildOf (Utilities|GetClass OtherActor) "/Game/Blueprints/Pawns/BP_Player.BP_Player_C")
      ;[1 1 1] If the colliding actor is a player, and there's no dialogue active, then trigger the dialogue from this object, and then destroy this object
      (Class|BPIDialogueInterface|TriggerDialogue(Message) _dialoguemanager (Variables|Default|GetDialogueToTrigger))
      (Actor|DestroyActor))))

(event EventBeginPlay
  (CallFunction|CheckforDialogueManager))

(fn ConstructionScript)

(fn CheckforDialogueManager
  ;[1 1 1] Checking for an existing dialogue manager in the scene. If one doesn't exist, print to the console, and destroy this object.
  (bind _returnvalue (Actor|GetActorOfClass "/Game/Blueprints/Dialogue/BP_DialogueManager.BP_DialogueManager_C"))
  (if (!= _returnvalue 0)
    (Variables|Default|SetDialogueManager _returnvalue)
    (else
      (Development|PrintString (Utilities|String|Append (Utilities|GetObjectName self) " cannot find Dialogue Manager") true true "(R=1.000000,G=0.000000,B=0.000000,A=1.000000)")
      (Actor|DestroyActor))))