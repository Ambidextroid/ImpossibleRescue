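; Dialogue manager Blueprint that plays linear conversations from a data table in a dialogue widget created at BeginPlay.
; TriggerDialogue stores the table, shows the widget and displays the entry at the current index, printing an error if none is found.
; Each update sets speaker name, text and portrait and plays optional 2D audio.
; ProgressDialogue steps through rows in order, removing the widget and resetting the index after the last.
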(event EventBeginPlay
  (CallFunction|InitializeDialogueWidget))

(event EventTriggerDialogue
  (params (DialogueToTrigger :type Data%20Table%20Object%20Reference))
  (Variables|Default|SetCurrentDialogueTable DialogueToTrigger)
  (CallFunction|OpenDialogue))

(event EventProgressDialogue
  (CallFunction|StepDialogue))

(fn ConstructionScript)

(fn InitializeDialogueWidget
  ;[1 1 1] Creating the dialogue widget
  (bind _returnvalue (UserInterface|CreateWidget "/Game/Blueprints/Widgets/WBP_DialogueWidget.WBP_DialogueWidget_C"))
  (Variables|Default|SetDialogueWidget _returnvalue))

(fn OpenDialogue
  ;[1 1 1] Add to viewport, then retrieve the dialogue entry
  (UserInterface|Viewport|AddtoViewport (Variables|Default|GetDialogueWidget) 0)
  (bind (_dialoguefound _speaker _speakerimage _dialoguetext _dialogueaudio) (CallFunction|GetNextDialogueEntry))
  ;[1 1 1] As long as the dialogue is found, update the dialogue, else print error
  (if _dialoguefound
    (CallFunction|UpdateDialogue _speaker _speakerimage _dialoguetext _dialogueaudio)
    (Variables|Default|SetIsDialogueActive true)
    (else
      (Development|PrintString "Dialogue Not Found" true true "(R=1.000000,G=0.026519,B=0.000000,A=1.000000)"))))

(fn EndDialogue
  ;[1 1 1] Remove the widget from the viewport, reset the dialogue index, and set dialogue active to false
  (Widget|RemovefromParent (Variables|Default|GetDialogueWidget))
  (Variables|Default|SetCurrentDialogueIndex 0)
  (Variables|Default|SetIsDialogueActive false))

(fn GetNextDialogueEntry
  (bind _currentdialogueindex (Variables|Default|GetCurrentDialogueIndex))
  (bind _currentdialoguetable (Variables|Default|GetCurrentDialogueTable))
  ;[1 1 1] Getting all the data rows by name, then checking that the current index doesn't exceed the length of the returned array
  (bind _outrownames (DataTable|GetDataTableRowNames _currentdialoguetable))
  (if (< _currentdialogueindex (Utilities|Array|Length _outrownames))
    ;[1 1 1] Get the row by the name previously found, break the structure, and return the results
    (bind _returnvalue (Utilities|GetDataTableRow _currentdialoguetable (Utilities|Array|Get(acopy) _outrownames _currentdialogueindex))
      (:then
        (return true (Utilities|String|EnumtoString (.Speaker (Utilities|Struct|BreakF_DialogueStructure _returnvalue))) (.SpeakerImage (Utilities|Struct|BreakF_DialogueStructure _returnvalue)) (.DialogueText (Utilities|Struct|BreakF_DialogueStructure _returnvalue)) (.DialogueAudio (Utilities|Struct|BreakF_DialogueStructure _returnvalue)))))
    (else
      ;[1 1 1] If we've exceeded the array index length, return with the bool dialogue found as false
      (return false "" 0 "" 0))))

(fn UpdateDialogue
  (params (Speaker :type String) (SpeakerImage :type Texture%202D%20Object%20Reference) (DialogueText :type String) (DialogueAudio :type Sound%20Cue%20Object%20Reference))
  (bind _dialoguewidget (Variables|Default|GetDialogueWidget))
  ;[1 1 1] Setting the speaker name, dialogue text, and speaker imager to the results given in the parameter, then checking if dialogue audio is valid, and playing it if it is
  (Rendering|Components|TextRender|SetText (Variables|/Game/Blueprints/Widgets/WBP_DialogueWidget.WBP_DialogueWidget_C|GetSpeakerName _dialoguewidget) (Utilities|Text|ToText(String) Speaker))
  (Rendering|Components|TextRender|SetText (Variables|/Game/Blueprints/Widgets/WBP_DialogueWidget.WBP_DialogueWidget_C|GetDialogueText _dialoguewidget) (Utilities|Text|ToText(String) DialogueText))
  (Appearance|SetBrushfromTexture (Variables|/Game/Blueprints/Widgets/WBP_DialogueWidget.WBP_DialogueWidget_C|GetSpeakerImage _dialoguewidget) SpeakerImage false)
  (if (!= DialogueAudio 0)
    (Audio|PlaySound2D DialogueAudio 1.0 1.0 0.0 0 0)))

(fn StepDialogue
  ;[1 1 1] Increment to next index, then get the data entry results
  (Math|Integer|IncrementInt (Variables|Default|GetCurrentDialogueIndex)
    (:%20%20
      (bind (_dialoguefound _speaker _speakerimage _dialoguetext _dialogueaudio) (CallFunction|GetNextDialogueEntry))
      ;[1 1 1] If dialogue is found, update the dialogue, else end the dialogue
      (if _dialoguefound
        (CallFunction|UpdateDialogue _speaker _speakerimage _dialoguetext _dialogueaudio)
        (else
          (CallFunction|EndDialogue))))))