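; An interactable actor that starts a dialogue message when its Interacted event fires.
; On BeginPlay it finds the level's BP_DialogueManager, or prints an error and destroys itself if none exists.
; On interaction it confirms player pawn 0 is a BP_Player and sends DialogueToTrigger to the manager unless dialogue is already active.
; The trigger is not destroyed after use, despite its inline comment.
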(event Custom|StartDialogue
  (bind _dialoguemanager (Variables|Default|GetDialogueManager))
  ;[1 1 1] Check if the colliding actor is a player, and whether dialogue is already active
  (Utilities|Casting|CastToBP_Player (Game|Player|GetPlayerPawn 0))
  (if (not (Variables|/Game/Blueprints/Dialogue/BP_DialogueManager.BP_DialogueManager_C|GetIsDialogueActive _dialoguemanager))
    ;[1 1 1] If the colliding actor is a player, and there's no dialogue active, then trigger the dialogue from this object, and then destroy this object
    (Class|BPIDialogueInterface|TriggerDialogue(Message) _dialoguemanager (Variables|Default|GetDialogueToTrigger))))

(event EventBeginPlay
  (CallFunction|CheckforDialogueManager))

(event EventInteracted
  (CallFunction|StartDialogue))

(fn ConstructionScript)

(fn CheckforDialogueManager
  ;[1 1 1] Checking for an existing dialogue manager in the scene. If one doesn't exist, print to the console, and destroy this object.
  (bind _returnvalue (Actor|GetActorOfClass "/Game/Blueprints/Dialogue/BP_DialogueManager.BP_DialogueManager_C"))
  (if (!= _returnvalue 0)
    (Variables|Default|SetDialogueManager _returnvalue)
    (else
      (Development|PrintString (Utilities|String|Append (Utilities|GetObjectName self) " cannot find Dialogue Manager") true true "(R=1.000000,G=0.000000,B=0.000000,A=1.000000)")
      (Actor|DestroyActor))))