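; BP_Door_Sliding is a sliding mechanism door that opens when its linked Trigger fires.
; On BeginPlay it binds to the Trigger's OnTriggered event if one is valid, which calls Open.
; Open plays a heavy mechanical sound at the door and runs a timeline that lerps the mesh sideways along local Y.
; The opening is one-way, as the actor destroys itself when the timeline finishes.
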(event Custom|Open
  (Audio|PlaySoundatLocation "/Game/Audio/SoundWaves/Temp/SFX/421722__lowpolygon__heavy-mechancial-door-open_Cue.421722__lowpolygon__heavy-mechancial-door-open_Cue" (Transformation|GetActorLocation) "0, 0, 0" 1.0 1.0 0.0 0 0 0)
  (bind _newtrack_0 (Timeline|DoorOpeningTimeline Play)
    (:Update
      (Transformation|SetRelativeLocation (Variables|Default|GetDoorMesh) (Math|Vector|Lerp(Vector) "0, 0, 0" "0,-150.000000, 0" _newtrack_0) false false))
    (:Finished
      (Actor|DestroyActor))))

(event EventBeginPlay
  (bind _trigger (Variables|Default|GetTrigger))
  (Utilities|IsValid _trigger
    (:Is%20Valid
      (EventDispatchers|BindEventtoOnTriggered _trigger (delegate EventInteracted)))))

(event EventInteracted
  (CallFunction|Open))

(fn ConstructionScript)