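; BP_Door is a button-operated door that the player's shadow opens, after which it sinks and removes itself.
; It binds to the player's door interact dispatcher and, if the button is in range, sends the button mesh to the shadow and waits for its opening time.
; It then disables the button, removes its outline, plays a sound, changes its colour and lowers the door via a Timeline lerp before destroying the actor.
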(event Custom|DoorInteract
  (bind _playerreference (Variables|Default|GetPlayerReference))
  (bind _button (Variables|Default|GetButton))
  (bind _shadowreference (Variables|/Game/Blueprints/Pawns/BP_Player.BP_Player_C|GetShadowReference _playerreference))
  (bind _outlinemesh (Variables|/Game/Blueprints/Mechanisms/Doors/BP_DoorButton.BP_DoorButton_C|GetOutlineMesh _button))
  ;[1 1 1] Button is pushed
  (if (not (Variables|Default|GetAnimating))
    (if (Variables|/Game/Blueprints/Mechanisms/Doors/BP_DoorButton.BP_DoorButton_C|GetInRange (Variables|Default|GetButton))
      ;[1 1 1] Send button location to shadow
      (Variables|Default|SetAnimating true)
      (Default|DoorOpen _shadowreference (Variables|/Game/Blueprints/Mechanisms/Doors/BP_DoorButton.BP_DoorButton_C|GetButtonMesh (Variables|Default|GetButton)))
      (Utilities|FlowControl|Delay (Variables|/Game/PlayerCharacter/BP_Shadow.BP_Shadow_C|GetDoorOpeningTime _shadowreference))
      ;[1 1 1] Destroy button outline
      (Variables|/Game/Blueprints/Mechanisms/Doors/BP_DoorButton.BP_DoorButton_C|SetUsable _button false)
      (if (Utilities|IsValid _outlinemesh)
        (Components|DestroyComponent _outlinemesh)
        (Audio|PlaySoundatLocation (Variables|Default|GetDoorOpenSound) (Transformation|GetActorLocation) "0, 0, 0" 1.0 1.0 0.0 0 0 0)
        ;[1 1 1] Open door
        (Default|ChangeColour (Variables|Default|GetButton))
        (bind _output_get (Variables|Default|SetStartLocation (Transformation|GetWorldLocation (Variables|Default|GetDefaultSceneRoot))))
        (bind _newtrack_0 (Timeline|Timeline_0 Play)
          (:Update
            (Transformation|SetWorldLocation (Variables|Default|GetDefaultSceneRoot) (Math|Vector|Lerp(Vector) _output_get (+ _output_get "0, 0,-300.000000") _newtrack_0) false false))
          (:Finished
            (Actor|DestroyActor)))))))

(event EventBeginPlay
  ;[1 1 1] Button is pushed
  (bind _asbp_player (Utilities|Casting|CastToBP_Player (Game|GetPlayerCharacter 0)))
  (bind _output_get (Variables|Default|SetPlayerReference _asbp_player))
  (EventDispatchers|BindEventtoDoorInteractDispatcher _output_get (delegate Custom|DoorInteract)))

(fn ConstructionScript)