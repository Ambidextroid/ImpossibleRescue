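; BP_DoorButton is a door button that highlights itself when an interaction collider enters its trigger.
; If usable, overlap by a component tagged InteractCollider sets InRange and spawns a scaled-up duplicate mesh with an outline material on every slot.
; Leaving the trigger clears InRange and destroys the duplicate.
; A ChangeColour event swaps the outline to an alternate material; press handling is absent from this graph.
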(event OnComponentBeginOverlap(ButtonCollider)
  (params (OverlappedComponent :type Primitive%20Component%20Object%20Reference) (OtherActor :type Actor%20Object%20Reference) (OtherComp :type Primitive%20Component%20Object%20Reference) (OtherBodyIndex :type Integer) (bFromSweep :type Boolean) (SweepResult :type Hit%20Result%20Structure%20%28by%20ref%29))
  (bind _staticmesh (Variables|Default|GetStaticMesh))
  (bind _returnvalue (Transformation|GetRelativeTransform _staticmesh))
  ;[1 1 1] Check if button can be pushed
  (if (Components|ComponentHasTag OtherComp "InteractCollider")
    (if (Variables|Default|GetUsable)
      (Variables|Default|SetInRange true)
      ;[1 1 1] Outline button
      ;;[1 1 1] Duplicate button mesh and increase size
      (bind _returnvalue_2 (AddComponent|AddStaticMeshComponent false (Math|Transform|MakeTransform (.location _returnvalue) (.rotation _returnvalue) (* (.scale _returnvalue) (Variables|Default|GetOutlineSale)))))
      (bind _output_get (Variables|Default|SetOutlineMesh _returnvalue_2))
      (Components|StaticMesh|SetStaticMesh _output_get (Variables|/Script/Engine.StaticMeshComponent|GetStaticMesh (Variables|Default|GetStaticMesh)))
      ;;[1 1 1] Set duplicate to outline material
      (for _index (range 0 (- (Utilities|Array|Length (Rendering|Material|GetMaterials (Variables|Default|GetOutlineMesh))) 1))
        (Rendering|Material|SetMaterial (Variables|Default|GetOutlineMesh) _index "/Game/Blueprints/Mechanisms/Doors/MI_ButtonOutline.MI_ButtonOutline")))))

(event OnComponentEndOverlap(ButtonCollider)
  (params (OverlappedComponent :type Primitive%20Component%20Object%20Reference) (OtherActor :type Actor%20Object%20Reference) (OtherComp :type Primitive%20Component%20Object%20Reference) (OtherBodyIndex :type Integer))
  (bind _outlinemesh (Variables|Default|GetOutlineMesh))
  ;[1 1 1] Check if button can be pushed
  (if (Components|ComponentHasTag OtherComp "InteractCollider")
    (Variables|Default|SetInRange false)
    ;[1 1 1] Outline button
    (if (Utilities|IsValid _outlinemesh)
      (Components|DestroyComponent _outlinemesh))))

(event Custom|ChangeColour
  ;[1 1 1] Outline button
  (for _index (range 0 (- (Utilities|Array|Length (Rendering|Material|GetMaterials (Variables|Default|GetOutlineMesh))) 1))
    (Rendering|Material|SetMaterial (Variables|Default|GetOutlineMesh) _index "/Game/Blueprints/Mechanisms/Doors/MI_ButtonOutline1.MI_ButtonOutline1")))

(fn ConstructionScript)