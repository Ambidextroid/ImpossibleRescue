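; BP_Door_Disappearing is a door mechanism that sinks out of the way and then removes itself from the level.
; On BeginPlay it binds Disappear to an optional Trigger's OnTriggered event, and its Interacted event calls Disappear directly.
; Disappear plays a timeline that lerps the Cube's relative location straight down, then destroys the actor when finished.
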(event Custom|Disappear
  (bind _newtrack_0 (Timeline|Timeline_0 PlayFromStart)
    (:Update
      (Transformation|SetRelativeLocation (Variables|Default|GetCube) (Math|Vector|Lerp(Vector) "0, 0, 0" "0,0.000000,-300.000000" _newtrack_0) false false))
    (:Finished
      (Actor|DestroyActor))))

(event EventBeginPlay
  (bind _trigger (Variables|Default|GetTrigger))
  (Utilities|IsValid _trigger
    (:Is%20Valid
      (EventDispatchers|BindEventtoOnTriggered _trigger (delegate Custom|Disappear)))))

(event EventInteracted
  (CallFunction|Disappear))

(fn ConstructionScript)