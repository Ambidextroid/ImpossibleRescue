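; BP_Switch_Simple is a switch that forwards Interacted to a linked Interactable, with optional locked start and single use.
; When locked, an Interacted call only unlocks it; otherwise it triggers the valid target, then locks if UseOnce is set.
; Unlock changes the sphere's collision object type, while Lock disables its collision without setting IsLocked.
; Both recolor the point light to show the state.
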(event Custom|Unlock
  (Collision|SetCollisionObjectType (Variables|Default|GetSphere) "ECC_GameTraceChannel6")
  (Rendering|Components|Light|SetLightColor (Variables|Default|GetPointLight) (Variables|Default|GetOpenColor) true))

(event Custom|Lock
  (Collision|SetCollisionEnabled (Variables|Default|GetSphere) "NoCollision")
  (Rendering|Components|Light|SetLightColor (Variables|Default|GetPointLight) (Variables|Default|GetLockColor) true))

(event EventBeginPlay
  (if (not (Variables|Default|GetIsLocked))
    (CallFunction|Unlock)))

(event Collision|EventActorBeginOverlap
  (params (OtherActor :type Actor%20Object%20Reference)))

(event EventTick
  (params (DeltaSeconds :type Float%20%28single-precision%29)))

(event EventInteracted
  (if (Variables|Default|GetIsLocked)
    (Variables|Default|SetIsLocked false)
    (CallFunction|Unlock)
    (else
      (Utilities|IsValid (Utilities|ToObject(Interface) (Variables|Default|GetInteractable))
        (:Is%20Valid
          (Default|Interacted (Variables|Default|GetInteractable))
          (if (Variables|Default|GetUseOnce)
            (CallFunction|Lock)))))))

(fn ConstructionScript)