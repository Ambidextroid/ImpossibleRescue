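; BP_Switch_Simple_HealthSpawn is a simple switch variant that rewards the player with a health pickup when unlocked.
; On Unlock it runs the parent logic, spawns a BP_Health actor at the HealthSpawn transform, and makes a platform mesh visible.
; All other events and the construction script only defer to the parent or are disabled, so switch behaviour is inherited.
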(event EventBeginPlay
  (|CallParentFunction) ; This node is disabled and will not be called.\nDrag off pins to build functionality.
)

(event Collision|EventActorBeginOverlap
  (params (OtherActor :type Actor%20Object%20Reference))
  (|CallParentFunction OtherActor) ; This node is disabled and will not be called.\nDrag off pins to build functionality.
)

(event EventTick
  (params (DeltaSeconds :type Float%20%28single-precision%29))
  (|CallParentFunction DeltaSeconds) ; This node is disabled and will not be called.\nDrag off pins to build functionality.
)

(event EventUnlock
  (|CallParentFunction)
  (Game|SpawnActorfromClass "/Game/Pickups/BP_Health.BP_Health_C" (Math|Conversions|ToTransform(Vector) (Variables|Default|GetHealthSpawn)) "Undefined" 0 0)
  (Rendering|SetVisibility (Variables|/Game/Blueprints/Mechanisms/Platforms/BP_MovingPlatform.BP_MovingPlatform_C|GetPlatform (Variables|Default|GetPlatform)) true false))

(fn ConstructionScript
  (|CallParentFunction))