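; Moving platform that oscillates continuously between the positions of referenced Origin and Destination actors.
; At BeginPlay it caches both locations and derives a time modifier from path length and Speed, making one full round trip last distance divided by Speed.
; Each Tick maps a sine of elapsed time onto the path and sets the location without sweep, easing at both ends and starting from the midpoint.
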(event EventBeginPlay
  (Variables|Default|SetLocation1 (Transformation|GetActorLocation (Variables|Default|GetOrigin)))
  (Variables|Default|SetLocation2 (Transformation|GetActorLocation (Variables|Default|GetDestination)))
  (Variables|Default|SetMovementPath (- (Variables|Default|GetLocation2) (Variables|Default|GetLocation1)))
  (CallFunction|CalculateTimeModifier))

(event EventTick
  (params (DeltaSeconds :type Float%20%28single-precision%29))
  (Variables|Default|SetTimeElasped (+ (Variables|Default|GetTimeElasped) (Utilities|Time|GetWorldDeltaSeconds)))
  (Transformation|SetActorLocation (+ (Variables|Default|GetLocation1) (* (Variables|Default|GetMovementPath) (/ (+ (Math|Trig|Sin(Degrees) (* (* (Variables|Default|GetTimeElasped) 3.6e+02) (Variables|Default|GetTimeModifier))) 1.0) 2.0))) false false))

(fn ConstructionScript)

(fn CalculateTimeModifier
  (bind _output_get (LocalVariables|SetTime (/ (Math|Vector|VectorLength (Variables|Default|GetMovementPath)) (Variables|Default|GetSpeed))))
  (Variables|Default|SetTimeModifier (/ 1.0 _output_get)))