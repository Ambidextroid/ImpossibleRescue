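; Pistol weapon that fires BP_Projectile from its arrow and shows a laser sight.
; Trigger pull spawns a shot with sound and starts a fire-rate timeline whose shots check overheat, spend player ammo and add heat, using the player's SMG stats.
; A second timeline drives the sight, line-tracing horizontally to set its end point and hiding it when the mouse nears screen centre.
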(event EventBeginPlay
  (bind _returnvalue (Game|GetPlayerController 0))
  (bind _sight (Variables|Default|GetSight))
  (bind _arrow (Variables|Default|GetArrow))
  (bind _sight_2 (Variables|Default|GetSight))
  (bind (_locationx _locationy) (Game|Player|GetMousePosition _returnvalue))
  (bind _returnvalue_2 (Transformation|GetWorldRotation _arrow))
  (bind _returnvalue_3 (Transformation|GetWorldLocation _sight))
  (bind (_sizex _sizey) (HUD|GetViewportSize _returnvalue))
  (bind _returnvalue_4 (Math|Rotator|GetRotationXVector _returnvalue_2))
  (bind (_x _y _z) (Math|Vector|BreakVector _returnvalue_3))
  (bind _returnvalue_5 (* _returnvalue_4 5e+03))
  (bind _returnvalue_6 (+ (Math|Vector|MakeVector _x _y 0.0) _returnvalue_5))
  (|CallParentFunction)
  (Components|Timeline|SetPlayRate (Variables|Default|GetPistolFireRate) (/ 1.0 (Variables|/Game/Blueprints/Pawns/BP_Player.BP_Player_C|GetSMGFireRate (Variables|Default|GetPlayerReference))))
  ;[1 1 1] Laser sight
  (Timeline|Update Play
    (:Update
      (if (|((((pow((x-h),2))/(pow(w,2)))+(pow((y-v),2)))<(pow(r,2))) _locationx (+ (/ (Math|Conversions|ToFloat(Integer) _sizex) 2.0) 0.0) _locationy (+ (/ (Math|Conversions|ToFloat(Integer) _sizey) 2.0) 0.0) 8e+01 1.0)
        (Development|SetHiddeninGame _sight_2 true false)
        (else
          (Development|SetHiddeninGame _sight_2 false false)
          (bind _outhit (Collision|LineTraceByChannel (Math|Vector|MakeVector _x _y _z) (Math|Vector|MakeVector (.x _returnvalue_6) (.y _returnvalue_6) _z) "TraceTypeQuery2" false 0 "None" true "(R=0.000000,G=0.034457,B=1.000000,A=1.000000)" "(R=1.000000,G=0.718554,B=0.099455,A=1.000000)"))
          (if (Class|KismetMathLibrary|EqualExactlyVectorVector (.location _outhit) "0, 0, 0")
            (Effects|Components|ParticleSystem|SetVectorParameter (Variables|Default|GetSight) "SightEnd" (- (Math|Vector|MakeVector (.x _returnvalue_6) (.y _returnvalue_6) _z) (Transformation|GetWorldLocation (Variables|Default|GetSight))))
            (else
              (Effects|Components|ParticleSystem|SetVectorParameter (Variables|Default|GetSight) "SightEnd" (- (.location _outhit) (Transformation|GetWorldLocation (Variables|Default|GetSight)))))))))))

(event Collision|EventActorBeginOverlap
  (params (OtherActor :type Actor%20Object%20Reference))
  (|CallParentFunction OtherActor) ; This node is disabled and will not be called.\nDrag off pins to build functionality.
)

(event EventTick
  (params (DeltaSeconds :type Float%20%28single-precision%29))
  (|CallParentFunction DeltaSeconds) ; This node is disabled and will not be called.\nDrag off pins to build functionality.
)

(event EventOnTriggerPull
  (bind _arrow (Variables|Default|GetArrow))
  (bind _playerreference (Variables|Default|GetPlayerReference))
  (bind _playerreference_2 (Variables|Default|GetPlayerReference))
  (bind _playerreference_3 (Variables|Default|GetPlayerReference))
  (bind _arrow_2 (Variables|Default|GetArrow))
  (bind _returnvalue (Transformation|GetWorldTransform _arrow_2))
  (bind _returnvalue_2 (Transformation|GetWorldTransform _arrow))
  (bind _smgammocost (Variables|/Game/Blueprints/Pawns/BP_Player.BP_Player_C|GetSMGAmmoCost _playerreference_3))
  ;[1 1 1] Fire projectile
  (if (> (Variables|/Game/Blueprints/Pawns/BP_Player.BP_Player_C|GetAmmo (Variables|Default|GetPlayerReference)) 0)
    (Utilities|FlowControl|Sequence
      (:then_0
        (Timeline|PistolFireRate PlayFromStart
          (:Fire
            (if (and (not (Variables|/Game/Blueprints/Pawns/BP_Player.BP_Player_C|GetOverheated _playerreference)) (> (Variables|/Game/Blueprints/Pawns/BP_Player.BP_Player_C|GetAmmo _playerreference) 0))
              (Game|SpawnActorfromClass "/Game/PlayerCharacter/Weapons/PistolProjectile/BP_Projectile.BP_Projectile_C" (Math|Transform|MakeTransform (.location _returnvalue) (.rotation _returnvalue) "0.500000,0.100000,0.100000") "Undefined" 0 0)
              (bind _output_get (Variables|/Game/Blueprints/Pawns/BP_Player.BP_Player_C|SetAmmo _playerreference_3 (- (Variables|/Game/Blueprints/Pawns/BP_Player.BP_Player_C|GetAmmo _playerreference_3) _smgammocost)))
              (Default|CallPlayerAmmoUpdated _playerreference_2 _output_get)
              (Default|AddHeat _playerreference_2 _smgammocost)))))
      (:then_1
        (Game|SpawnActorfromClass "/Game/PlayerCharacter/Weapons/PistolProjectile/BP_Projectile.BP_Projectile_C" (Math|Transform|MakeTransform (.location _returnvalue_2) (.rotation _returnvalue_2) "0.500000,0.100000,0.100000") "Undefined" 0 0)
        (Audio|PlaySound2D "/Game/Audio/SoundWaves/Temp/SFX/tmp_pistolLight_Cue.tmp_pistolLight_Cue" 1.0 1.0 0.0 0 0)))))

(event EventOnTriggerRelease
  (bind _playerreference (Variables|Default|GetPlayerReference))
  (bind _playerreference_2 (Variables|Default|GetPlayerReference))
  (bind _playerreference_3 (Variables|Default|GetPlayerReference))
  (bind _arrow (Variables|Default|GetArrow))
  (bind _returnvalue (Transformation|GetWorldTransform _arrow))
  (bind _smgammocost (Variables|/Game/Blueprints/Pawns/BP_Player.BP_Player_C|GetSMGAmmoCost _playerreference_3))
  ;[1 1 1] Fire projectile
  (Timeline|PistolFireRate Stop
    (:Fire
      (if (and (not (Variables|/Game/Blueprints/Pawns/BP_Player.BP_Player_C|GetOverheated _playerreference)) (> (Variables|/Game/Blueprints/Pawns/BP_Player.BP_Player_C|GetAmmo _playerreference) 0))
        (Game|SpawnActorfromClass "/Game/PlayerCharacter/Weapons/PistolProjectile/BP_Projectile.BP_Projectile_C" (Math|Transform|MakeTransform (.location _returnvalue) (.rotation _returnvalue) "0.500000,0.100000,0.100000") "Undefined" 0 0)
        (bind _output_get (Variables|/Game/Blueprints/Pawns/BP_Player.BP_Player_C|SetAmmo _playerreference_3 (- (Variables|/Game/Blueprints/Pawns/BP_Player.BP_Player_C|GetAmmo _playerreference_3) _smgammocost)))
        (Default|CallPlayerAmmoUpdated _playerreference_2 _output_get)
        (Default|AddHeat _playerreference_2 _smgammocost)))))

(fn ConstructionScript
  (|CallParentFunction))