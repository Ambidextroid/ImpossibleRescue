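; Laser weapon that fires a continuous damaging beam from its FirePoint while the trigger is held.
; Trigger pull spawns beam and spark particles plus a looped-until-release 2D sound, then runs an initial line trace.
; While firing, Tick re-traces to reposition both effects and applies frame-time-scaled damage, without updating spark visibility on misses.
; Trigger release tears down the effects and sound; CheckForEnemyCollision is an empty stub.
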(event EventBeginPlay
  (|CallParentFunction) ; This node is disabled and will not be called.\nDrag off pins to build functionality.
)

(event Collision|EventActorBeginOverlap
  (params (OtherActor :type Actor%20Object%20Reference))
  (|CallParentFunction OtherActor) ; This node is disabled and will not be called.\nDrag off pins to build functionality.
)

(event EventTick
  (params (DeltaSeconds :type Float%20%28single-precision%29))
  (|CallParentFunction DeltaSeconds)
  (if (Variables|Default|GetIsFiring)
    (CallFunction|UpdateEmitterPositions)))

(event EventOnTriggerPull
  (bind _firepoint (Variables|Default|GetFirePoint))
  (bind _returnvalue (Transformation|GetWorldLocation _firepoint))
  (Utilities|FlowControl|Sequence
    (:then_0
      (bind _returnvalue_2 (Effects|SpawnEmitterAttached "/Game/Particles/P_ShadowGunLaser.P_ShadowGunLaser" (Variables|Default|GetFirePoint) "None"))
      (Variables|Default|SetLaser%20Particle _returnvalue_2)
      (Variables|Default|SetLaserSpawn true))
    (:then_1
      (bind _returnvalue_3 (Effects|SpawnEmitteratLocation "/Game/Particles/P_ShadowGunLaserSparks.P_ShadowGunLaserSparks" "0, 0, 0"))
      (Variables|Default|SetHit%20Particle _returnvalue_3)
      (Variables|Default|SetLaserHitSpawn true))
    (:then_2
      (bind (_outhit _returnvalue_4) (Collision|LineTraceByChannel _returnvalue (+ _returnvalue (* (Math|Vector|GetForwardVector _firepoint) (Variables|Default|GetLaserDistance))) "TraceTypeQuery5" true 0 "None"))
      (if _returnvalue_4
        (Rendering|SetVisibility (Variables|Default|GetHit%20Particle) true false)
        (bind _output_get (Variables|Default|SetHitPoint (.Location (Collision|BreakHitResult _outhit))))
        (Transformation|SetWorldLocation (Variables|Default|GetHit%20Particle) _output_get false false)
        (Game|Damage|ApplyDamage (.HitActor (Collision|BreakHitResult _outhit)) (* (Variables|Default|GetDamagePerTick) (Utilities|Time|GetWorldDeltaSeconds)) 0 0)
        (else
          (Rendering|SetVisibility (Variables|Default|GetHit%20Particle) false false))))
    (:then_3
      (Class|ParticleSystemComponent|SetBeamSourcePoint (Variables|Default|GetLaser%20Particle) 0 _returnvalue)
      (Class|ParticleSystemComponent|SetBeamEndPoint (Variables|Default|GetLaser%20Particle) 0 (Variables|Default|GetHitPoint))
      (Variables|Default|SetIsFiring true))
    (:then_4
      (bind _returnvalue_5 (Audio|SpawnSound2D "/Game/Audio/SoundWaves/Temp/SFX/laserSound_Cue.laserSound_Cue" 1.0 1.0 0.0 0))
      (Variables|Default|SetBeamSound _returnvalue_5))))

(event EventOnTriggerRelease
  (bind _hit_particle (Variables|Default|GetHit%20Particle))
  (Utilities|FlowControl|Sequence
    (:then_0
      (if (Variables|Default|GetLaserSpawn)
        (Variables|Default|SetLaserSpawn false)
        (Components|DestroyComponent (Variables|Default|GetLaser%20Particle))))
    (:then_1
      (if (Variables|Default|GetLaserHitSpawn)
        (Utilities|IsValid _hit_particle
          (:Is%20Valid
            (Components|Activation|Deactivate _hit_particle)
            (Variables|Default|SetLaserHitSpawn false)
            (Variables|Default|SetIsFiring false)))))
    (:then_2
      (Audio|Components|Audio|Stop (Variables|Default|GetBeamSound)))))

(fn ConstructionScript
  (|CallParentFunction))

(fn UpdateEmitterPositions
  (bind _laser_particle (Variables|Default|GetLaser%20Particle))
  (bind _firepoint (Variables|Default|GetFirePoint))
  (bind _returnvalue (Transformation|GetWorldLocation _firepoint))
  (bind _outhit (Collision|LineTraceByChannel _returnvalue (+ _returnvalue (* (Math|Vector|GetForwardVector _firepoint) (Variables|Default|GetLaserDistance))) "TraceTypeQuery5" true 0 "None"))
  (Class|ParticleSystemComponent|SetBeamSourcePoint _laser_particle 0 _returnvalue)
  (Class|ParticleSystemComponent|SetBeamEndPoint _laser_particle 0 (.Location (Collision|BreakHitResult _outhit)))
  (Transformation|SetWorldLocation (Variables|Default|GetHit%20Particle) (.Location (Collision|BreakHitResult _outhit)) false false)
  (Game|Damage|ApplyDamage (.HitActor (Collision|BreakHitResult _outhit)) (* (Variables|Default|GetDamagePerTick) (Utilities|Time|GetWorldDeltaSeconds)) 0 0))

(fn CheckforEnemyCollision)