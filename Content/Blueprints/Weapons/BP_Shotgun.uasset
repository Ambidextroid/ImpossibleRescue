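; Shotgun weapon that, on trigger pull with ammo available, plays a Niagara effect and fire sound and damages enemies inside a cone.
; HitCone collision switches on only during the shot to gather overlapping BP_EnemyBase actors.
; A visibility trace from Arrow to each enemy supplies the hit distance for unclamped linear damage falloff.
; Damage applies whatever the trace hits, and ammo is not decremented here.
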(event EventBeginPlay
  (|CallParentFunction)
  (Collision|SetCollisionEnabled (Variables|Default|GetHitCone) "NoCollision"))

(event Collision|EventActorBeginOverlap
  (params (OtherActor :type Actor%20Object%20Reference))
  (|CallParentFunction OtherActor) ; This node is disabled and will not be called.\nDrag off pins to build functionality.
)

(event EventTick
  (params (DeltaSeconds :type Float%20%28single-precision%29))
  (|CallParentFunction DeltaSeconds) ; This node is disabled and will not be called.\nDrag off pins to build functionality.
)

(event EventOnTriggerPull
  (bind _hitcone (Variables|Default|GetHitCone))
  (bind _emitterpoint (Variables|Default|GetEmitterPoint))
  (bind _returnvalue (Transformation|GetWorldTransform _emitterpoint))
  ;[1 1 1] Damage enemies
  (if (> (Variables|/Game/Blueprints/Pawns/BP_Player.BP_Player_C|GetAmmo (Variables|Default|GetPlayerReference)) 0)
    (Niagara|SpawnSystematLocation "/Game/PlayerCharacter/Weapons/NS_Shotgun.NS_Shotgun" (.location _returnvalue) (.rotation _returnvalue))
    (Audio|PlaySound2D (Variables|Default|GetFireSound) 1.0 1.0 0.0 0 0)
    (Collision|SetCollisionEnabled _hitcone "QueryOnly")
    (for _array_element (Collision|GetOverlappingActors _hitcone "/Game/Enemies/BP_EnemyBase.BP_EnemyBase_C" :!class /Script/Engine.PrimitiveComponent)
      (bind _outhit (Collision|LineTraceByChannel (Transformation|GetWorldLocation (Variables|Default|GetArrow)) (Transformation|GetActorLocation _array_element) "TraceTypeQuery1" false 0 "None"))
      (Game|Damage|ApplyDamage _array_element (|((((NegativeOne*x)+dist)/dist)*dmg) (.distance _outhit) 6e+02 7e+01 -1.0) 0 0))
    (Collision|SetCollisionEnabled (Variables|Default|GetHitCone) "NoCollision")))

(fn ConstructionScript
  (|CallParentFunction))