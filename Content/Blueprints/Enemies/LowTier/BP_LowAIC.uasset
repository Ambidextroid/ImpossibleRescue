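; AI controller for the low-tier enemy that turns it toward the player and fires projectiles while it is activated.
; On possession it caches the enemy; each tick with line of sight it rotates the model and runs a delay-gated firing loop, with a random first-shot delay.
; Shots alternate between left and right fire points, aimed at the player.
; While the enemy is inactive, its health resets to default.
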(event Custom|Shoot
  (bind _returnvalue (Game|Player|GetPlayerPawn 0))
  (bind _enemyreference (Variables|Default|GetEnemyReference))
  (bind _returnvalue_2 (Transformation|GetActorLocation _returnvalue))
  (bind _rightfire (Variables|/Game/Blueprints/Enemies/LowTier/BP_LowEnemy.BP_LowEnemy_C|GetRightFire _enemyreference))
  (bind _returnvalue_3 (Transformation|GetWorldLocation _rightfire))
  ;[1 1 1] Shoot periodically when enemy senses player
  (if (Variables|/Game/Blueprints/Enemies/BP_EnemyBase.BP_EnemyBase_C|GetActivated (Variables|Default|GetEnemyReference))
    (bind _output_get (Variables|Default|SetLeftFire (not (Variables|Default|GetLeftFire))))
    (if _output_get
      (Game|SpawnActorfromClass "/Game/Enemies/LowTier/BP_LowEnemyProjectile.BP_LowEnemyProjectile_C" (Math|Transform|MakeTransform (Transformation|GetWorldLocation (Variables|/Game/Blueprints/Enemies/LowTier/BP_LowEnemy.BP_LowEnemy_C|GetLeftFire (Variables|Default|GetEnemyReference))) (Math|Conversions|RotationFromXVector (Math|Vector|GetUnitDirection(Vector) (Transformation|GetWorldLocation (Variables|/Game/Blueprints/Enemies/LowTier/BP_LowEnemy.BP_LowEnemy_C|GetLeftFire (Variables|Default|GetEnemyReference))) _returnvalue_2)) "0.500000,0.100000,0.100000") "Undefined" 0 0)
      (else
        (Game|SpawnActorfromClass "/Game/Enemies/LowTier/BP_LowEnemyProjectile.BP_LowEnemyProjectile_C" (Math|Transform|MakeTransform _returnvalue_3 (Math|Conversions|RotationFromXVector (Math|Vector|GetUnitDirection(Vector) _returnvalue_3 _returnvalue_2)) "0.500000,0.100000,0.100000") "Undefined" 0 0)))))

(event EventBeginPlay)

(event EventTick
  (params (DeltaSeconds :type Float%20%28single-precision%29))
  ;[1 1 1] Face player when line of sight
  (if (Variables|/Game/Blueprints/Enemies/BP_EnemyBase.BP_EnemyBase_C|GetActivated (Variables|Default|GetEnemyReference))
    (if (Controller|LineOfSightTo (Game|Player|GetPlayerPawn 0) "0, 0, 0" false)
      (Transformation|SetWorldRotation (Variables|/Game/Blueprints/Enemies/LowTier/BP_LowEnemy.BP_LowEnemy_C|GetModelRoot (Variables|Default|GetEnemyReference)) (Math|Conversions|RotationFromXVector (Math|Vector|GetUnitDirection(Vector) (Transformation|GetWorldLocation (Variables|/Script/Engine.Actor|GetRootComponent (Variables|Default|GetEnemyReference))) (Transformation|GetActorLocation (Game|Player|GetPlayerPawn 0)))) false false)
      ;[1 1 1] Shooting timing
      (if (not (Variables|Default|GetShooting))
        (Variables|Default|SetShooting true)
        (if (Variables|Default|GetFirstShot)
          (Utilities|FlowControl|Delay (Math|Random|RandomFloatinRange 0.0 0.5))
          (Variables|Default|SetFirstShot false))
        (CallFunction|Shoot)
        (Utilities|FlowControl|Delay (Variables|Default|GetFireDelay))
        (Variables|Default|SetShooting false)))
    (else
      (Variables|/Game/Blueprints/Enemies/BP_EnemyBase.BP_EnemyBase_C|SetHealth (Variables|Default|GetEnemyReference) (Variables|Default|GetDefault%20Health)))))

(event EventPossess
  (params (PossessedPawn :type Pawn%20Object%20Reference))
  (bind _asbp_low_enemy (Utilities|Casting|CastToBP_LowEnemy PossessedPawn))
  (Variables|Default|SetEnemyReference _asbp_low_enemy))

(fn ConstructionScript)