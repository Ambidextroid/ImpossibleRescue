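; Low-tier enemy Blueprint, a thin child class that relies on inherited logic for its teleport-in spawn.
; On BeginPlay it sets Model0 as the Primitive, runs the parent BeginPlay, then teleports in if Activated or otherwise hides the model.
; The Teleportin event just forwards to BaseTeleport, and the construction script only calls the parent.
; Tick and overlap events are disabled stubs.
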(event EventBeginPlay
  ;[1 1 1] Benet Plowden
  (Variables|Default|SetPrimitive (Variables|Default|GetModel_0))
  (|CallParentFunction)
  (if (Variables|Default|GetActivated)
    (CallFunction|Teleportin)
    (else
      (Rendering|SetVisibility (Variables|Default|GetModel_0) false false))))

(event Collision|EventActorBeginOverlap
  (params (OtherActor :type Actor%20Object%20Reference))
  (|CallParentFunction OtherActor) ; This node is disabled and will not be called.\nDrag off pins to build functionality.
)

(event EventTick
  (params (DeltaSeconds :type Float%20%28single-precision%29))
  (|CallParentFunction DeltaSeconds) ; This node is disabled and will not be called.\nDrag off pins to build functionality.
)

(event EventTeleportin
  ;[1 1 1] Benet Plowden
  (CallFunction|BaseTeleport))

(fn ConstructionScript
  (|CallParentFunction))