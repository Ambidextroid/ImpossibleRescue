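; Base enemy Blueprint that handles damage, death and teleport-in activation.
; Lethal damage fires the OnDeath dispatcher, plays effects and destroys the actor, randomly dropping ammo when the player is low.
; ActivateEnemy calls TeleportIn, a placeholder print here, then delays activation so attacks wait for visibility.
; BaseTeleport, not called here, swaps a static or skeletal mesh's materials for a Timeline-driven sphere-mask reveal, then restores them.
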(event Custom|ActivateEnemy
  ;[1 1 1] Benet Plowden: when an enemy is teleported in, trigger the shader effect and a sound
  (CallFunction|Teleportin)
  (Audio|PlaySoundatLocation "/Game/Audio/SoundWaves/SFX/SC_Teleport.SC_Teleport" (Transformation|GetActorLocation) "0, 0, 0" 1.0 1.0 0.0 0 0 0)
  ;;[1 1 1] Delay needed or enemy will attack before becoming completely visible
  (Utilities|FlowControl|Delay 1.0)
  (Variables|Default|SetActivated true))

(event Custom|BaseTeleport
  (bind _primitive (Variables|Default|GetPrimitive))
  (bind _primitive_2 (Variables|Default|GetPrimitive))
  ;[1 1 1] Benet Plowden: The 'teleport in' shader effect
  ;;[1 1 1] Make sure the mesh is actually visible
  (Rendering|SetVisibility (Variables|Default|GetPrimitive) true false)
  ;;[1 1 1] Make a note of your original materials
  (bind _asstatic_mesh_component (Utilities|Casting|CastToStaticMeshComponent _primitive_2)
    (:then
      (Variables|Default|SetOriginalMaterials (Rendering|Material|GetMaterials _asstatic_mesh_component)))
    (:CastFailed
      (bind _asskeletal_mesh_component (Utilities|Casting|CastToSkeletalMeshComponent _primitive_2))
      (Variables|Default|SetOriginalMaterials (Rendering|Material|GetMaterials _asskeletal_mesh_component))))
  ;;[1 1 1] Set all the material slots to use the teleportation effect material
  (for (_ _array_index) (Variables|Default|GetOriginalMaterials)
    (Rendering|Material|SetMaterial (Variables|Default|GetPrimitive) _array_index "/Game/Materials/Test/Mat_Teleport_Inst.Mat_Teleport_Inst")
    ;;[1 1 1] Create an increasingly large radius for the SphereMask in the teleportation shader to use
    (bind _radius (Timeline|Timeline_0 Play)
      (:Update
        (bind _asstatic_mesh_component_2 (Utilities|Casting|CastToStaticMeshComponent _primitive)
          (:then
            (Rendering|Material|SetScalarParameterValueonMaterials _asstatic_mesh_component_2 "Radius" (* _radius (.SphereRadius (Collision|GetComponentBounds (Variables|Default|GetPrimitive))))))
          (:CastFailed
            (bind _asskeletal_mesh_component_2 (Utilities|Casting|CastToSkeletalMeshComponent _primitive))
            (Rendering|Material|SetScalarParameterValueonMaterials _asskeletal_mesh_component_2 "Radius" (* _radius (.SphereRadius (Collision|GetComponentBounds (Variables|Default|GetPrimitive))))))))
      (:Finished
        ;;[1 1 1] Revert to original materials
        (for (_array_element _array_index_2) (Variables|Default|GetOriginalMaterials)
          (Rendering|Material|SetMaterial (Variables|Default|GetPrimitive) _array_index_2 _array_element))))))

(event Game|Damage|EventAnyDamage
  (params (Damage :type Float%20%28single-precision%29) (DamageType :type Damage%20Type%20Object%20Reference) (InstigatedBy :type Controller%20Object%20Reference) (DamageCauser :type Actor%20Object%20Reference))
  (bind _returnvalue (Transformation|GetActorLocation))
  ;[1 1 1] Benet Plowden: apply damage and fire off event dispatcher if dead
  (Variables|Default|SetHealth (- (Variables|Default|GetHealth) Damage))
  (if (<= (Variables|Default|GetHealth) 0.0)
    (Default|CallOnDeath)
    ;[0.9219 0.101 0.04407] Dante
    (Audio|PlaySoundatLocation (Variables|Default|GetExplosionSound) _returnvalue "0, 0, 0" 1.0 1.0 0.0 0 0 0)
    (Audio|PlaySoundatLocation (Variables|Default|GetDeathSound) _returnvalue "0, 0, 0" 1.0 1.0 0.0 0 0 0)
    (Effects|SpawnEmitteratLocation "/Game/Particles/P_EnemyExplosion.P_EnemyExplosion" _returnvalue)
    (bind _asbp_player (Utilities|Casting|CastToBP_Player (Game|Player|GetPlayerPawn 0)))
    (if (and (< (Variables|/Game/Blueprints/Pawns/BP_Player.BP_Player_C|GetAmmo _asbp_player) 20) (Math|Random|RandomBool))
      (Game|SpawnActorfromClass "/Game/Pickups/BP_Ammo.BP_Ammo_C" (Math|Conversions|ToTransform(Vector) _returnvalue) "Undefined" 0 0)
      (Actor|DestroyActor)
      (else
        (Actor|DestroyActor)))))

(fn ConstructionScript)

(fn Teleportin
  (Development|PrintString "Hello"))