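; AI controller for the high-tier enemy BP_HighEnemy, handling roaming and shooting at the player.
; While the enemy is activated, MoveCycle chains moves to random nearby navigable points.
; Tick turns the model toward a visible player and triggers cooldown-gated Shoot bursts, randomly delaying the first.
; Each burst fires three aimed projectiles from alternating left and right muzzles; inactive enemies have their health reset every tick.
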(event Custom|MoveCycle
  ;[1 1 1] Immediately move to random location and repeat
  (if (Variables|/Game/Blueprints/Enemies/BP_EnemyBase.BP_EnemyBase_C|GetActivated (Variables|Default|GetEnemyReference))
    (AI|AIMoveTo 0 (.RandomLocation (Class|NavigationSystemV1|GetRandomPointinNavigableRadius (Transformation|GetWorldLocation (Variables|/Script/Engine.Actor|GetRootComponent (Variables|Default|GetEnemyReference))) 5e+02 0 0)) 0 5.0 false
      (:OnSuccess
        _)
      (:OnFail
        _))
    (CallFunction|MoveCycle)))

(event Custom|Shoot
  (bind _returnvalue (Game|Player|GetPlayerPawn 0))
  (bind _enemyreference (Variables|Default|GetEnemyReference))
  (bind _enemyreference_2 (Variables|Default|GetEnemyReference))
  (bind _returnvalue_2 (Transformation|GetActorLocation _returnvalue))
  (bind _leftfire (Variables|/Game/Blueprints/Enemies/HIghTier/BP_HighEnemy.BP_HighEnemy_C|GetLeftFIre _enemyreference_2))
  (bind _rightfire (Variables|/Game/Blueprints/Enemies/HIghTier/BP_HighEnemy.BP_HighEnemy_C|GetRightFire _enemyreference))
  (bind _returnvalue_3 (Transformation|GetWorldLocation _leftfire))
  (bind _returnvalue_4 (Transformation|GetWorldLocation _rightfire))
  ;[1 1 1] Shoot periodically when enemy senses player
  (if (Variables|Default|GetMoving)
    _
    (else
      (CallFunction|MoveCycle)
      (Variables|Default|SetMoving true)))
  (Utilities|FlowControl|Sequence
    (:then_0
      _)
    (:then_1
      (Utilities|FlowControl|Delay (Variables|Default|GetBurstDelay)))
    (:then_2
      (Utilities|FlowControl|Delay (* (Variables|Default|GetBurstDelay) 2.0))))
  (bind _output_get (Variables|Default|SetShootLeft (not (Variables|Default|GetShootLeft))))
  (if _output_get
    (Game|SpawnActorfromClass "/Game/Enemies/HighTier/BP_HighEnemyProjectile.BP_HighEnemyProjectile_C" (Math|Transform|MakeTransform _returnvalue_3 (Math|Conversions|RotationFromXVector (Math|Vector|GetUnitDirection(Vector) _returnvalue_3 _returnvalue_2)) "0.200000,0.100000,0.100000") "Undefined" 0 0)
    (else
      (Game|SpawnActorfromClass "/Game/Enemies/HighTier/BP_HighEnemyProjectile.BP_HighEnemyProjectile_C" (Math|Transform|MakeTransform _returnvalue_4 (Math|Conversions|RotationFromXVector (Math|Vector|GetUnitDirection(Vector) _returnvalue_4 _returnvalue_2)) "0.200000,0.100000,0.100000") "Undefined" 0 0))))

(event EventBeginPlay
  ;[1 1 1] Immediately move to random location and repeat
  (Utilities|FlowControl|Delay 0.2)
  (CallFunction|MoveCycle))

(event EventTick
  (params (DeltaSeconds :type Float%20%28single-precision%29))
  ;[1 1 1] Face player when line of sight
  (if (Variables|/Game/Blueprints/Enemies/BP_EnemyBase.BP_EnemyBase_C|GetActivated (Variables|Default|GetEnemyReference))
    (if (Controller|LineOfSightTo (Game|Player|GetPlayerPawn 0) "0, 0, 0" false)
      (Transformation|SetWorldRotation (Variables|/Game/Blueprints/Enemies/HIghTier/BP_HighEnemy.BP_HighEnemy_C|GetModelRoot (Variables|Default|GetEnemyReference)) (Math|Conversions|RotationFromXVector (Math|Vector|GetUnitDirection(Vector) (Transformation|GetWorldLocation (Variables|/Script/Engine.Actor|GetRootComponent (Variables|Default|GetEnemyReference))) (Transformation|GetActorLocation (Game|Player|GetPlayerPawn 0)))) false false)
      ;[1 1 1] Shooting timing
      (if (not (Variables|Default|GetShooting))
        (Variables|Default|SetShooting true)
        (if (Variables|Default|GetFirstShot)
          (Utilities|FlowControl|Delay (Math|Random|RandomFloatinRange 0.0 0.5))
          (Variables|Default|SetFirstShot false))
        (CallFunction|Shoot)
        (Utilities|FlowControl|Delay (Variables|Default|GetFireDelay))
        (Variables|Default|SetShooting false)))
    (else
      (Variables|/Game/Blueprints/Enemies/BP_EnemyBase.BP_EnemyBase_C|SetHealth (Variables|Default|GetEnemyReference) (Variables|Default|GetDefault%20Health)))))

(event EventPossess
  (params (PossessedPawn :type Pawn%20Object%20Reference))
  (bind _asbp_high_enemy (Utilities|Casting|CastToBP_HighEnemy PossessedPawn))
  (Variables|Default|SetEnemyReference _asbp_high_enemy))

(fn ConstructionScript)