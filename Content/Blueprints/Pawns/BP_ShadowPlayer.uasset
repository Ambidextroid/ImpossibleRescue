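; Player pawn variant that can carry an overheating laser gun in place of the parent's SMG, switched by the HasLaserGun flag.
; The primary weapon spawn and fire overrides either attach and trigger BP_Laser or fall back to parent logic.
; While the laser fires, Tick adds heat, broadcasts the update and, at the maximum, plays an overheat cue and releases the trigger.
; Firing stays blocked while overheated.
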(event EventBeginPlay
  (|CallParentFunction) ; This node is disabled and will not be called.\nDrag off pins to build functionality.
)

(event Collision|EventActorBeginOverlap
  (params (OtherActor :type Actor%20Object%20Reference)))

(event EventTick
  (params (DeltaSeconds :type Float%20%28single-precision%29))
  (if (Variables|Default|GetHasLaserGun)
    (CallFunction|LaserGunUpdate)))

(event EventOnWeaponFired
  (params (Weapon :type BP%20Base%20Weapon%20Object%20Reference) (AmmoCost :type Integer))
  ;[1 1 1] If no laser gun, run the original weapon fire logic, else continue with laser gun logic
  (if (Variables|Default|GetHasLaserGun)
    (if (not (Variables|Default|GetOverheated))
      (Default|OnTriggerPull Weapon))
    (else
      (|CallParentFunction (Variables|Default|GetWeapon1) (Variables|Default|GetSMGAmmoCost)))))

(fn ConstructionScript
  (|CallParentFunction))

(fn SpawnLaserGun
  (bind _weapon1spawn (Variables|Default|GetWeapon1Spawn))
  (bind _returnvalue (Transformation|GetWorldTransform _weapon1spawn))
  ;[1 1 1] Overidden function to spawn laser gun instead of smg. Uses same logic, just with laser gun class
  (bind _returnvalue_2 (Game|SpawnActorfromClass "/Game/Blueprints/Weapons/BP_Laser.BP_Laser_C" (Math|Transform|MakeTransform (.location _returnvalue) (.rotation _returnvalue) "1,1,1") "AlwaysSpawn" 0 0))
  (bind _output_get (Variables|Default|SetWeapon1 _returnvalue_2))
  (bind _asbp_laser (Utilities|Casting|CastToBP_Laser _output_get))
  (bind _output_get_2 (Variables|Default|SetLaserGun _asbp_laser))
  (Transformation|AttachComponentToComponent _output_get_2 (Variables|Default|GetWeapon1Spawn) "None" "SnapToTarget" "SnapToTarget" "KeepRelative" true))

(fn SpawnPrimaryWeapon
  ;[1 1 1] Decides whether to spawn laser gun, or the (parent function) smg based on the bool
  (if (Variables|Default|GetHasLaserGun)
    (CallFunction|SpawnLaserGun)
    (else
      (|CallParentFunction))))

(fn AddHeatasFloat
  (params (Heat :type Float%20%28single-precision%29))
  (bind _output_get (LocalVariables|SetUnclampedHeat (+ (Variables|Default|GetHeat) (* (Variables|Default|GetHeatPerShot) Heat))))
  ;[1 1 1] Perform comparison before clamping to max heat in case of precision errors with float comparison
  (bind _output_get_2 (Variables|Default|SetOverheated (>= _output_get (Variables|Default|GetMaxHeat))))
  (if _output_get_2
    (Audio|PlaySound2D "/Game/Audio/SoundWaves/Temp/SFX/overheat_Cue.overheat_Cue" 1.0 1.0 0.0 0 0))
  ;[1 1 1] Clamp heat to max heat
  (bind _output_get_3 (Variables|Default|SetHeat (Math|Float|Min(Float) (LocalVariables|GetUnclampedHeat) (Variables|Default|GetMaxHeat))))
  (Default|CallWeaponHeatUpdated _output_get_3 (Variables|Default|GetOverheated))
  (CallFunction|HeatAdded))

(fn LaserGunUpdate
  (bind _lasergun (Variables|Default|GetLaserGun))
  ;[1 1 1] Function for updating the laser gun when firing. Adds heat based on the float variable
  (if (Variables|/Game/Blueprints/Weapons/BP_Laser.BP_Laser_C|GetIsFiring _lasergun)
    (CallFunction|AddHeatasFloat (Variables|Default|GetLaserHeatPerTick))
    (if (Variables|Default|GetOverheated)
      (Default|OnTriggerRelease _lasergun))))