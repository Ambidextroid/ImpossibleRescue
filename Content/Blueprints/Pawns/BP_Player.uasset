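; Player character for a top-down shooter, with cursor aiming, a dash that shields against damage, health, pausing and game over.
; BeginPlay spawns overridable weapons, an optional shadow drone and the UI widgets.
; Firing spends shared ammo and builds heat, which can lock both weapons until a delayed cooldown drains it.
; Interact advances active dialogue first, otherwise messages the overlapped interactable, gated by the drone's following state.
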(event OnComponentBeginOverlap(InteractSphere)
  (params (OverlappedComponent :type Primitive%20Component%20Object%20Reference) (OtherActor :type Actor%20Object%20Reference) (OtherComp :type Primitive%20Component%20Object%20Reference) (OtherBodyIndex :type Integer) (bFromSweep :type Boolean) (SweepResult :type Hit%20Result%20Structure%20%28by%20ref%29))
  ;[1 1 1] Add interact prompt and set currently selected interactable object if in range
  (UserInterface|Viewport|AddtoViewport (Variables|UI|GetInteractPrompt) 0)
  (Variables|Default|SetInteractable OtherActor))

(event OnComponentEndOverlap(InteractSphere)
  (params (OverlappedComponent :type Primitive%20Component%20Object%20Reference) (OtherActor :type Actor%20Object%20Reference) (OtherComp :type Primitive%20Component%20Object%20Reference) (OtherBodyIndex :type Integer))
  ;[1 1 1] Add interact prompt and set currently selected interactable object if in range
  (Widget|RemovefromParent (Variables|UI|GetInteractPrompt))
  (Variables|Default|SetInteractable 0))

(event Custom|HealthPickup
  (params (AddedHealth :type Float%20%28single-precision%29))
  ;[0.4235 1 0.5915] Health and Damage
  ;;[0.9826 1 0.8673] Add health
  (if (Variables|PlayerState|GetVulnerable)
    ;;;[1 1 1] Add health
    (bind _output_get (Variables|Health|SetHealth (Math|Float|Clamp(Float) (+ AddedHealth (Variables|Health|GetHealth)) 0.0 (Variables|Health|GetMaxHealth))))
    ;;;[1 1 1] Update UI
    (Default|CallPlayerHealthUpdated (/ _output_get (Variables|Health|GetMaxHealth)))))

(event Custom|AmmoPickup
  (params (AddedAmmo :type Integer))
  ;[1 0.07396 0.07396] Shooting
  ;;[1 1 1] Add ammo
  (bind _output_get (Variables|Shooting|SetAmmo (+ AddedAmmo (Variables|Shooting|GetAmmo))))
  (Default|CallPlayerAmmoUpdated _output_get))

(event Custom|AddGameOverWidget
  ;[0.4235 1 0.5915] Health and Damage
  ;;[1 1 1] Wait for animation to play, then create game over menu
  (Utilities|FlowControl|Delay 1.5)
  (bind _returnvalue (UserInterface|CreateWidget "/Game/Blueprints/Widgets/WBP_GameOverMenu.WBP_GameOverMenu_C"))
  (UserInterface|Viewport|AddtoViewport _returnvalue 0))

(event Custom|DashEnded
  ;[1 0.9084 0.21] Movement
  ;;[1 1 1] Dashing
  (Dashing|EndDash)
  (Variables|PlayerState|SetShielded false)
  (Utilities|FlowControl|Delay (Variables|Dashing|GetDashCoolDown))
  (Variables|Dashing|SetDashRecovered true))

(event Custom|OnWeaponFired
  (params (Weapon :type BP%20Base%20Weapon%20Object%20Reference) (AmmoCost :type Integer))
  ;[1 0.07396 0.07396] Shooting
  ;;[1 1 1] Fire Weapon
  (if (not (Variables|Shooting|GetOverheated))
    (if (>= (- (Variables|Shooting|GetAmmo) AmmoCost) 0)
      (Default|OnTriggerPull Weapon)
      ;;;[1 1 1] Reduce ammo by ammo cost
      (bind _output_get (Variables|Shooting|SetAmmo (- (Variables|Shooting|GetAmmo) AmmoCost)))
      (Default|CallPlayerAmmoUpdated _output_get)
      (Shooting|AddHeat AmmoCost)
      (else
        (Audio|PlaySound2D "/Game/Audio/SoundWaves/Temp/SFX/noAmmo_Cue.noAmmo_Cue" 1.0 1.0 0.0 0 0)))))

(event Custom|OnFiringStopped
  (params (Weapon :type BP%20Base%20Weapon%20Object%20Reference))
  ;[1 0.07396 0.07396] Shooting
  ;;[1 1 1] Stop Firing
  (Default|OnTriggerRelease Weapon))

(event Custom|HeatAdded
  ;[1 0.07396 0.07396] Shooting
  ;;[1 1 1] Control heat cooldown process
  (Utilities|FlowControl|Sequence
    (:then_0
      (Timeline|Cooldown Stop
        (:Update
          (Shooting|ReduceHeat))))
    (:then_1
      (Utilities|FlowControl|RetriggerableDelay (Math|Float|SelectFloat (Variables|Default|GetOverheatCooldownDelay) (Variables|Default|GetStandardCooldownDelay) (Variables|Shooting|GetOverheated)))
      (Timeline|Cooldown PlayFromStart))))

(event Custom|CooldownComplete
  ;[1 0.07396 0.07396] Shooting
  ;;[1 1 1] Control heat cooldown process
  (Timeline|Cooldown Stop
    (:Update
      (Shooting|ReduceHeat))))

(event Custom|AimDirectionEvent
  (params (Direction :type Vector))
  (bind _returnvalue (Math|Conversions|RotationFromXVector (Math|Vector|MakeVector (.x Direction) (.y Direction) 0.0)))
  (bind _returnvalue_2 (Game|GetPlayerController 0))
  (bind _weapon1spawn (Variables|Default|GetWeapon1Spawn))
  (bind _hitresult (Game|Player|GetHitResultUnderCursorbyChannel _returnvalue_2 "TraceTypeQuery3" true))
  (bind _returnvalue_3 (Transformation|GetWorldLocation _weapon1spawn))
  (bind _returnvalue_4 (Math|Vector|GetUnitDirection(Vector) _returnvalue_3 (.location _hitresult)))
  ;[1 0.9084 0.21] Movement
  (if (Variables|PlayerState|GetCanMove)
    (Transformation|SetWorldRotation (Variables|Collision|GetCapsuleComponent) _returnvalue false false)
    (Transformation|SetWorldRotation (Variables|Default|GetWeapon2Spawn) _returnvalue false false)
    (if (<= (Class|KismetMathLibrary|DegAcos (Math|Vector|DotProduct (Math|Vector|Normalize (Math|Vector|MakeVector (.x Direction) (.y Direction) 0.0)) (Math|Vector|Normalize (Math|Vector|MakeVector (.x _returnvalue_4) (.y _returnvalue_4) 0.0)))) 2e+01)
      (Transformation|SetWorldRotation _weapon1spawn (Math|Conversions|RotationFromXVector (Math|Vector|MakeVector (.x _returnvalue_4) (.y _returnvalue_4) 0.0)) false false))))

(event Custom|OnGameOver
  (Health|Die))

(event Custom|Unpaused
  ;[0 0.8904 1] Initial Setup
  ;;[1 1 1] Set UP Unpause Event
  (CallFunction|TogglePause))

(event EventBeginPlay
  (bind _charactermovement (Variables|Character|GetCharacterMovement))
  ;[0 0.8904 1] Initial Setup
  (Utilities|FlowControl|Sequence
    (:then_0
      ;;[1 1 1] Spawn shadow drone
      ;; Note from Dean: Added check if bp should have shadow drone, since player shadow bp inherits from this
      (if (Variables|Default|GetHasShadowDrone)
        (bind _returnvalue (Game|SpawnActorfromClass "/Game/PlayerCharacter/BP_Shadow.BP_Shadow_C" (Math|Transform|MakeTransform (Transformation|GetWorldLocation (Variables|Collision|GetCapsuleComponent)) "0, 0, 0" "1,1,1") "Undefined" 0 0))
        (Variables|Default|SetShadowReference _returnvalue)))
    (:then_1
      ;;[1 1 1] Note from Dean: Turned the spawn weapon logic into their own functions, and added a bool to easily turn on/off the secondary. Also, being their own functions means the child bp can override and potentially have different weapons
      ;;;[1 1 1] Spawn SMG
      (CallFunction|SpawnPrimaryWeapon))
    (:then_2
      ;;;[1 1 1] Spawn Shotgun
      (if (Variables|Shooting|GetHasSecondaryWeapon)
        (CallFunction|SpawnSecondaryWeapon)))
    (:then_3
      ;;[1 1 1] Set Up HUD
      (bind _returnvalue_2 (UserInterface|CreateWidget "/Game/Blueprints/Widgets/WBP_PlayerHUD.WBP_PlayerHUD_C" 0 self))
      (UserInterface|Viewport|AddtoViewport _returnvalue_2 0)
      (Variables|Default|SetPlayerHUD _returnvalue_2)
      (Default|CallPlayerHealthUpdated (/ (Variables|Health|GetHealth) (Variables|Health|GetMaxHealth)))
      (Default|CallPlayerAmmoUpdated (Variables|Shooting|GetAmmo))
      (bind _returnvalue_3 (UserInterface|CreateWidget "/Game/Blueprints/Widgets/WBP_InteractPrompt.WBP_InteractPrompt_C"))
      (Variables|UI|SetInteractPrompt _returnvalue_3)
      (bind _returnvalue_4 (UserInterface|CreateWidget "/Game/Blueprints/Widgets/WBP_DamageIndicator.WBP_DamageIndicator_C"))
      (UserInterface|Viewport|AddtoViewport _returnvalue_4 0)
      (Variables|Default|SetDamageIndicator _returnvalue_4))
    (:then_4
      ;;[1 1 1] Set up dash
      ;;;[1 1 1] Note default speed
      (Variables|Dashing|SetDefaultSpeed (Variables|/Script/Engine.CharacterMovementComponent|GetMaxWalkSpeed _charactermovement))
      (Variables|Dashing|SetDefaultAcceleration (Class|CharacterMovementComponent|GetMaxAcceleration _charactermovement))
      ;;;[1 1 1] Calculate required dash speed to cover distance
      (Variables|Dashing|SetDashSpeed (/ (Variables|Dashing|GetDashDistance) (Variables|Dashing|GetDashDuration))))
    (:then_5
      ;;[1 1 1] Set UP Unpause Event
      (bind _returnvalue_5 (UserInterface|CreateWidget "/Game/Blueprints/Widgets/WBP_PauseMenu.WBP_PauseMenu_C"))
      (Variables|UI|SetPauseMenu _returnvalue_5)
      (bind _asbp_game_mode_base (Utilities|Casting|CastToBP_GameModeBase (Game|GetGameMode)))
      (EventDispatchers|BindEventtoGameUnpausedDispatcher _asbp_game_mode_base (delegate Custom|Unpaused)))
    (:then_6
      (bind _asbp_game_mode_base_2 (Utilities|Casting|CastToBP_GameModeBase (Game|GetGameMode)))
      (EventDispatchers|BindEventtoGameOverDispatcher _asbp_game_mode_base_2 (delegate Custom|OnGameOver)))
    (:then_7
      (Variables|Shooting|SetHeatPerShot (/ 1.0 (Math|Conversions|ToFloat(Integer) (Variables|Shooting|GetShotsBeforeOverheat)))))))

(event Game|Damage|EventAnyDamage
  (params (Damage :type Float%20%28single-precision%29) (DamageType :type Damage%20Type%20Object%20Reference) (InstigatedBy :type Controller%20Object%20Reference) (DamageCauser :type Actor%20Object%20Reference))
  ;[0.4235 1 0.5915] Health and Damage
  ;;[1 1 1] Player damage
  ;;;[1 1 1] If the player can be hurt
  (if (and (not (Variables|PlayerState|GetShielded)) (Variables|PlayerState|GetVulnerable))
    ;;;[1 1 1] Reduce Health
    (bind _output_get (Variables|Health|SetHealth (- (Variables|Health|GetHealth) Damage)))
    ;;;[1 1 1] Update UI
    (Default|CallPlayerHealthUpdated (/ _output_get (Variables|Health|GetMaxHealth)))
    (Default|OnHurt (Variables|Default|GetDamageIndicator))
    ;;;[1 1 1] Check if dead
    (if (<= (Variables|Health|GetHealth) 0.0)
      (Health|Die))))

(event Input|ActionEvents|InputActionEscape
  (params (Key :type Key%20Structure))
  ;[0 0.8904 1] Initial Setup
  ;;[1 1 1] Set UP Unpause Event
  (:Pressed
    (CallFunction|TogglePause)))

(event Input|ActionEvents|InputActionWeapon1
  (params (Key :type Key%20Structure))
  (bind _weapon1 (Variables|Shooting|GetWeapon1))
  ;[1 0.07396 0.07396] Shooting
  ;;[1 1 1] Fire Weapons
  (:Pressed
    (CallFunction|OnWeaponFired _weapon1 (Variables|Shooting|GetSMGAmmoCost)))
  (:Released
    (CallFunction|OnFiringStopped _weapon1)))

(event Input|ActionEvents|InputActionInteract
  (params (Key :type Key%20Structure))
  (bind _interactable (Variables|Default|GetInteractable))
  ;[1 1 1] Interactions
  (:Pressed
    (bind _isdialogueactive (CallFunction|DialogueCheck))
    (if (not _isdialogueactive)
      (if (Variables|Default|GetHasShadow)
        (if (Variables|/Game/PlayerCharacter/BP_Shadow.BP_Shadow_C|GetFollowing (Variables|Default|GetShadowReference))
          (Default|CallDoorInteractDispatcher)
          (if (Utilities|IsValid _interactable) :!label _label
            (Class|IInteractable|Interacted(Message) _interactable)))
        (else
          (goto _label))))))

(event Input|ActionEvents|InputActionDash
  (params (Key :type Key%20Structure))
  ;[1 0.9084 0.21] Movement
  ;;[1 1 1] Dashing
  (:Pressed
    (if (and (Variables|Dashing|GetDashRecovered) (Variables|PlayerState|GetCanMove))
      (Variables|Dashing|SetDashRecovered false)
      (Variables|PlayerState|SetShielded true)
      (Dashing|StartDash)
      (Utilities|Time|SetTimerbyEvent (delegate Custom|DashEnded) (Variables|Dashing|GetDashDuration)))))

(event Input|ActionEvents|InputActionWeapon2
  (params (Key :type Key%20Structure))
  (bind _weapon2 (Variables|Shooting|GetWeapon2))
  (bind _hassecondaryweapon (Variables|Shooting|GetHasSecondaryWeapon))
  ;[1 0.07396 0.07396] Shooting
  ;;[1 1 1] Fire Weapons
  ;;;[1 1 1] Note from Dean: Added check here to stop secondary being fired if the bp doesn't have one
  (:Pressed
    (if _hassecondaryweapon
      (CallFunction|OnWeaponFired _weapon2 (Variables|Shooting|GetShotgunAmmoCost))))
  (:Released
    (if _hassecondaryweapon
      (CallFunction|OnFiringStopped _weapon2))))

(event Input|AxisEvents|InputAxisMoveForward
  (params (AxisValue :type Float%20%28single-precision%29))
  ;[1 0.9084 0.21] Movement
  ;;[1 1 1] Arrow key movement
  (Pawn|Input|AddMovementInput "1.000000,-1.000000, 0" AxisValue false))

(event Input|AxisEvents|InputAxisMoveRight
  (params (AxisValue :type Float%20%28single-precision%29))
  ;[1 0.9084 0.21] Movement
  ;;[1 1 1] Arrow key movement
  (Pawn|Input|AddMovementInput "1.000000,1.000000, 0" AxisValue false))

(fn ConstructionScript)

(fn Die
  (Input|DisableInput 0)
  (Variables|PlayerState|SetCanMove false)
  (Variables|PlayerState|SetVulnerable false)
  (Audio|PlaySound2D "/Game/Audio/SoundWaves/Temp/SFX/gameOver_Cue.gameOver_Cue" 1.0 1.0 0.0 0 0)
  (Variables|Health|SetHealth 0.0)
  (CallFunction|AddGameOverWidget))

(fn EndDash
  (bind _charactermovement (Variables|Character|GetCharacterMovement))
  (bind _charactermovement_2 (Variables|Character|GetCharacterMovement))
  (Variables|/Script/Engine.CharacterMovementComponent|SetMaxWalkSpeed _charactermovement (Variables|Dashing|GetDefaultSpeed))
  (Variables|/Script/Engine.CharacterMovementComponent|SetMaxAcceleration _charactermovement (Variables|Dashing|GetDefaultAcceleration))
  (Variables|/Script/Engine.CharacterMovementComponent|SetGravityScale _charactermovement_2 1.0)
  (Variables|/Script/Engine.MovementComponent|SetVelocity _charactermovement_2 (/ (Variables|/Script/Engine.MovementComponent|GetVelocity _charactermovement_2) 2.0)))

(fn StartDash
  (bind _charactermovement (Variables|Character|GetCharacterMovement))
  (Variables|/Script/Engine.CharacterMovementComponent|SetMaxWalkSpeed _charactermovement (Variables|Dashing|GetDashSpeed))
  (Variables|/Script/Engine.CharacterMovementComponent|SetMaxAcceleration _charactermovement (Variables|Dashing|GetMax%20Acceleration))
  (Audio|PlaySound2D "/Game/Audio/SoundWaves/Temp/SFX/dashSoundNew_Cue.dashSoundNew_Cue" 1.0 1.0 0.0 0 0)
  (Variables|/Script/Engine.CharacterMovementComponent|SetGravityScale (Variables|Character|GetCharacterMovement) 0.0))

(fn AddHeat
  (params (AmmoCount :type Integer))
  (bind _output_get (LocalVariables|SetUnclampedHeat (+ (Variables|Shooting|GetHeat) (* (Variables|Shooting|GetHeatPerShot) (Math|Conversions|ToFloat(Integer) AmmoCount)))))
  ;[1 1 1] Perform comparison before clamping to max heat in case of precision errors with float comparison
  (bind _output_get_2 (Variables|Shooting|SetOverheated (>= _output_get (Variables|Shooting|GetMaxHeat))))
  (if _output_get_2
    (Audio|PlaySound2D (Variables|Default|GetOverheatSound) 1.0 1.0 0.0 0 0))
  ;[1 1 1] Clamp heat to max heat
  (bind _output_get_3 (Variables|Shooting|SetHeat (Math|Float|Min(Float) (LocalVariables|GetUnclampedHeat) (Variables|Shooting|GetMaxHeat))))
  (Default|CallWeaponHeatUpdated _output_get_3 (Variables|Shooting|GetOverheated))
  (CallFunction|HeatAdded))

(fn ReduceHeat
  (bind _output_get (LocalVariables|SetBelowZero (< (- (Variables|Shooting|GetHeat) (* (Variables|Shooting|GetCooldownRate) (Utilities|Time|GetWorldDeltaSeconds))) 0.0)))
  ;[1 1 1] Can only still be overheated if was overheated on last frame and heat still above 0
  (Variables|Shooting|SetOverheated (and (Variables|Shooting|GetOverheated) (not _output_get)))
  (bind _output_get_2 (Variables|Shooting|SetHeat (Math|Float|Max(Float) (- (Variables|Shooting|GetHeat) (* (Variables|Shooting|GetCooldownRate) (Utilities|Time|GetWorldDeltaSeconds))) 0.0)))
  (Default|CallWeaponHeatUpdated _output_get_2 (Variables|Shooting|GetOverheated))
  (if (LocalVariables|GetBelowZero)
    (CallFunction|CooldownComplete)))

(fn TogglePause
  (bind _pausemenu (Variables|UI|GetPauseMenu))
  (bind _output_get (Variables|Default|SetGamePaused (not (Variables|Default|GetGamePaused))))
  (Game|SetGamePaused _output_get)
  (if (Variables|Default|GetGamePaused)
    (UserInterface|Viewport|AddtoViewport _pausemenu 0)
    (else
      (Widget|RemovefromParent _pausemenu))))

(fn SpawnPrimaryWeapon
  (bind _weapon1spawn (Variables|Default|GetWeapon1Spawn))
  (bind _returnvalue (Transformation|GetWorldTransform _weapon1spawn))
  (bind _returnvalue_2 (Game|SpawnActorfromClass "/Game/Blueprints/Weapons/BP_Pistol.BP_Pistol_C" (Math|Transform|MakeTransform (.location _returnvalue) (.rotation _returnvalue) "1,1,1") "AlwaysSpawn" 0 0))
  (bind _output_get (Variables|Shooting|SetWeapon1 _returnvalue_2))
  (Transformation|AttachComponentToComponent _output_get (Variables|Default|GetWeapon1Spawn) "None" "SnapToTarget" "SnapToTarget" "KeepRelative" true))

(fn SpawnSecondaryWeapon
  (bind _weapon1spawn (Variables|Default|GetWeapon1Spawn))
  (bind _returnvalue (Transformation|GetWorldTransform _weapon1spawn))
  (bind _returnvalue_2 (Game|SpawnActorfromClass "/Game/Blueprints/Weapons/BP_Shotgun.BP_Shotgun_C" (Math|Transform|MakeTransform (.location _returnvalue) (.rotation _returnvalue) "1,1,1") "AlwaysSpawn" 0 0))
  (bind _output_get (Variables|Shooting|SetWeapon2 _returnvalue_2))
  (Transformation|AttachComponentToComponent _output_get (Variables|Default|GetWeapon2Spawn) "None" "SnapToTarget" "SnapToTarget" "KeepRelative" true))

(fn DialogueCheck
  ;[1 1 1] Attempt to get dialogue manager in scene
  (bind _returnvalue (Actor|GetActorOfClass "/Game/Blueprints/Dialogue/BP_DialogueManager.BP_DialogueManager_C"))
  ;[1 1 1] If dialogue manager exists, continue, else return false. Using a temp variable for the bool since the get could return false after progressing dialogue
  (if (!= _returnvalue 0)
    (bind _output_get (LocalVariables|SetDialogueActive (Variables|/Game/Blueprints/Dialogue/BP_DialogueManager.BP_DialogueManager_C|GetIsDialogueActive _returnvalue)))
    ;[1 1 1] If dialogue is active, then progress the dialogue. Return the result either way.
    (if _output_get
      (Class|BPIDialogueInterface|ProgressDialogue(Message) _returnvalue))
    (return _output_get)
    (else
      (return false))))

(fn SetPlayerMesh)