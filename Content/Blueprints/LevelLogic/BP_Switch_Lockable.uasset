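; BP_Switch_Lockable is a level-logic switch that stays unusable until a linked Trigger fires.
; On BeginPlay it binds to the Trigger and sets its InteractSphere to ignore a custom trace channel.
; When triggered, it clears the Locked flag and restores overlap on that channel.
; Interactions are forwarded to the referenced Interactable only while unlocked.
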(event Custom|Unlocked
  ;[1 1 1] Unlock
  (Variables|Default|SetLocked false)
  (Collision|SetCollisionResponsetoChannel (Variables|Default|GetInteractSphere) "ECC_GameTraceChannel6" "ECR_Overlap"))

(event Custom|Lock
  (Collision|SetCollisionResponsetoChannel (Variables|Default|GetInteractSphere) "ECC_GameTraceChannel6" "ECR_Ignore"))

(event EventInteracted
  ;[1 1 1] Do smth. if unlocked and interacted with
  (if (not (Variables|Default|GetLocked))
    (Default|Interacted (Variables|Default|GetInteractable))))

(event EventBeginPlay
  ;[1 1 1] Bind to trigger
  (EventDispatchers|BindEventtoOnTriggered (Variables|Default|GetTrigger) (delegate Custom|Unlocked))
  (CallFunction|Lock))

(fn ConstructionScript)