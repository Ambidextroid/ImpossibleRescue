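; BP_LevelTrigger is a lockable box trigger that moves the player to the next level behind a screen fade.
; An interaction event clears its lock, and a Player-tagged overlap then asks BP_TransitionManager to begin fading.
; A looping timer polls the manager until the fade finishes, then clears itself, enables the loading screen and opens the NextLevel reference.
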(event OnComponentBeginOverlap(Box)
  (params (OverlappedComponent :type Primitive%20Component%20Object%20Reference) (OtherActor :type Actor%20Object%20Reference) (OtherComp :type Primitive%20Component%20Object%20Reference) (OtherBodyIndex :type Integer) (bFromSweep :type Boolean) (SweepResult :type Hit%20Result%20Structure%20%28by%20ref%29))
  (if (not (Variables|Default|GetLocked))
    (if (Actor|ActorHasTag OtherActor "Player")
      (CallFunction|BeginFade)
      (CallFunction|LoadonFadeComplete))))

(event EventBeginPlay)

(event Collision|EventActorBeginOverlap
  (params (OtherActor :type Actor%20Object%20Reference)))

(event EventTick
  (params (DeltaSeconds :type Float%20%28single-precision%29)))

(event EventInteracted
  (Variables|Default|SetLocked false))

(fn ConstructionScript)

(fn BeginFade
  ;[1 1 1] Tell the transition manager to begin fading
  (bind _returnvalue (Actor|GetActorOfClass "/Game/Blueprints/LevelLogic/BP_TransitionManager.BP_TransitionManager_C"))
  (Default|SettoFade _returnvalue "NewEnumerator1"))

(fn LoadonFadeComplete
  ;[1 1 1] Set a timer to keep checking until fade is complete
  (bind _returnvalue (Utilities|Time|SetTimerbyFunctionName 0 "CheckForFadeComplete" (Variables|Default|GetFadeCheckInterval) true))
  (Variables|Default|SetFadeTimerHandle _returnvalue))

(fn LoadNextLevel
  (Game|OpenLevel(byObjectReference) (Variables|Default|GetNextLevel)))

(fn CheckforFadeComplete
  ;[1 1 1] Keep asking the transition manager whether the fade is finished, then clear the timer handle, and load next level
  (bind _returnvalue (Actor|GetActorOfClass "/Game/Blueprints/LevelLogic/BP_TransitionManager.BP_TransitionManager_C"))
  (if (Variables|/Game/Blueprints/LevelLogic/BP_TransitionManager.BP_TransitionManager_C|GetIsFadeFinished _returnvalue)
    (Utilities|Time|ClearandInvalidateTimerbyHandle (Variables|Default|GetFadeTimerHandle))
    (Default|EnableLoadingScreen _returnvalue)
    (CallFunction|LoadNextLevel)))