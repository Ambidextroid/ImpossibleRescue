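; Transition manager that drives black-screen fades and shows a loading screen for level transitions.
; On BeginPlay it creates the fade overlay and loading widgets, and SetToFade adds the overlay to the viewport and starts a fade.
; Tick steps the overlay brush alpha by FadeRate times world delta seconds, then flags completion, removing the overlay only after fading in.
; EnableLoadingScreen adds the loading widget to the viewport.
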(event EventBeginPlay
  (CallFunction|CreateWidgets))

(event EventTick
  (params (DeltaSeconds :type Float%20%28single-precision%29))
  (CallFunction|FadeUpdate))

(fn ConstructionScript)

(fn CreateWidgets
  ;[1 1 1] Create the fade widget
  (bind _returnvalue (UserInterface|CreateWidget "/Game/Blueprints/Widgets/WBP_LevelTransitionFade.WBP_LevelTransitionFade_C"))
  (Variables|Default|SetOverlayWidget _returnvalue)
  ;[1 1 1] Create the loading screen widget
  (bind _returnvalue_2 (UserInterface|CreateWidget "/Game/Blueprints/Widgets/WBP_Loading.WBP_Loading_C"))
  (Variables|Default|SetLoadingWidget _returnvalue_2))

(fn FadeUpdate
  (LocalVariables|SetCurrentFade (.a (Variables|/Script/UMG.Border|GetBrushColor (Variables|/Game/Blueprints/Widgets/WBP_LevelTransitionFade.WBP_LevelTransitionFade_C|GetBlackScreenOverlay (Variables|Default|GetOverlayWidget)))))
  (switch Utilities|FlowControl|Switch|SwitchonE_FadeState (Variables|Default|GetFadeState)
    (:NewEnumerator0
      ;[1 1 1] Gradually fade in, then end the fade
      (if (<= (LocalVariables|GetCurrentFade) 0.0)
        (LocalVariables|SetCurrentFade 0.0)
        (CallFunction|EndFade true)
        (else
          (LocalVariables|SetCurrentFade (- (LocalVariables|GetCurrentFade) (CallFunction|DeltaFade))))))
    (:NewEnumerator1
      ;[1 1 1] Gradually fade out, then set state to stop fading
      (if (>= (LocalVariables|GetCurrentFade) 1.0)
        (LocalVariables|SetCurrentFade 1.0)
        (CallFunction|EndFade false)
        (else
          (LocalVariables|SetCurrentFade (+ (LocalVariables|GetCurrentFade) (CallFunction|DeltaFade)))))))
  (CallFunction|SetFadeAlpha (LocalVariables|GetCurrentFade)))

(fn SettoFade
  (params (FadeState :type E_FadeState%20Enum :default "NewEnumerator2"))
  ;[1 1 1] If state is being set to a fade, add to viewport
  (switch Utilities|FlowControl|Switch|SwitchonE_FadeState FadeState
    (:NewEnumerator0
      _)
    (:NewEnumerator1
      _))
  (UserInterface|Viewport|AddtoViewport (Variables|Default|GetOverlayWidget) 0)
  (Variables|Default|SetFadeState FadeState)
  (Variables|Default|SetIsFadeFinished false))

(fn EndFade
  (params (ShouldRemoveOverlay :type Boolean))
  ;[1 1 1] Function to finish fade and remove from viewport if needed
  (if ShouldRemoveOverlay
    (Widget|RemovefromParent (Variables|Default|GetOverlayWidget)))
  (Variables|Default|SetFadeState "NewEnumerator2")
  (Variables|Default|SetIsFadeFinished true))

(fn SetFadeAlpha
  (params (Alpha :type Float%20%28single-precision%29))
  (bind _overlaywidget (Variables|Default|GetOverlayWidget))
  (bind _blackscreenoverlay (Variables|/Game/Blueprints/Widgets/WBP_LevelTransitionFade.WBP_LevelTransitionFade_C|GetBlackScreenOverlay _overlaywidget))
  (bind _brushcolor (Variables|/Script/UMG.Border|GetBrushColor _blackscreenoverlay))
  ;[1 1 1] Simple function to set the alpha of the fade overlay
  (Class|Border|SetBrushColor _blackscreenoverlay (Utilities|Struct|MakeLinearColor (.r _brushcolor) (.g _brushcolor) (.b _brushcolor) Alpha)))

(fn DeltaFade
  (return (* (Variables|Default|GetFadeRate) (Utilities|Time|GetWorldDeltaSeconds))))

(fn EnableLoadingScreen
  (UserInterface|Viewport|AddtoViewport (Variables|Default|GetLoadingWidget) 0))