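; BP_Arena is a combat arena that fires OnTriggered and interacts its linked interactables once its enemy count reaches zero.
; At BeginPlay, a box overlap collects enemies and spawners, and each enemy's death event decrements the count.
; WakeEnemies activates placed enemies, while SpawnEnemies spawns, counts and activates new ones.
; The EnemiesSpawned flag is only set when already true, so it never blocks repeat spawns.
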(event Custom|CheckEnemies
  (bind _box (Variables|Default|GetBox))
  (Utilities|Array|Clear (Variables|Default|GetEnemyArray))
  (Utilities|Array|Clear (Variables|Default|GetSpawnerArray))
  (bind _outactors (Collision|BoxOverlapActors (Transformation|GetWorldLocation _box) (Components|Box|GetScaledBoxExtent _box) (Utilities|Array|MakeArray "ObjectTypeQuery2" "ObjectTypeQuery1") 0 :!class /Script/Engine.KismetSystemLibrary))
  (for _array_element _outactors
    (bind _asbp_enemy_base (Utilities|Casting|CastToBP_EnemyBase _array_element)
      (:then
        (Utilities|Array|Add (Variables|Default|GetEnemyArray) _asbp_enemy_base))
      (:CastFailed
        (bind _asbp_spawner_enemy (Utilities|Casting|CastToBP_Spawner_Enemy _array_element))
        (Utilities|Array|Add (Variables|Default|GetSpawnerArray) _asbp_spawner_enemy)))))

(event Custom|EnemyDestroyed
  (bind _enemycount (Variables|Default|GetEnemyCount))
  (Math|Integer|DecrementInt _enemycount
    (:%20%20
      (if (<= _enemycount 0)
        (Default|CallOnTriggered)
        (for _array_element (Variables|Default|GetInteractableArray)
          (Default|Interacted _array_element))))))

(event Custom|WakeEnemies
  (if (not (Variables|Default|GetEnemiesAwoken))
    (for _array_element (Variables|Default|GetEnemyArray)
      (Default|ActivateEnemy _array_element)
      (Variables|Default|SetEnemiesAwoken true))))

(event Custom|SpawnEnemies
  (if (Variables|Default|GetEnemiesSpawned)
    (Variables|Default|SetEnemiesSpawned true)
    (else
      (for _array_element (Variables|Default|GetSpawnerArray)
        (bind _newparam (Default|SpawninEnemy _array_element))
        (EventDispatchers|BindEventtoOnDeath _newparam (delegate Custom|EnemyDestroyed))
        (Math|Integer|IncrementInt (Variables|Default|GetEnemyCount)
          (:%20%20
            (Default|ActivateEnemy _newparam)))))))

(event EventBeginPlay
  (CallFunction|CheckEnemies)
  (Variables|Default|SetEnemyCount (Utilities|Array|Length (Variables|Default|GetEnemyArray)))
  (for _array_element (Variables|Default|GetEnemyArray)
    (EventDispatchers|BindEventtoOnDeath _array_element (delegate Custom|EnemyDestroyed))))

(fn ConstructionScript)