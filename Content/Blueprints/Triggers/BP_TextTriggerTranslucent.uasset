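; BP_TextTriggerTranslucent is a trigger actor that shows a text popup while another actor overlaps it.
; On BeginPlay it copies TriggerText into the WBP_TextPopup held by its TextWidget component, revealing it immediately if Showing is already set.
; Begin and end overlap call Reveal and Hide on that widget, using the Showing flag to skip redundant calls.
; Overlaps are not filtered by actor type or counted.
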(event EventBeginPlay
  ;[1 1 1] Set Widget Text
  (bind _aswbp_text_popup (Utilities|Casting|CastToWBP_TextPopup (UserInterface|GetWidget (Variables|Default|GetTextWidget))))
  (bind _output_get (Variables|Default|SetNotificationWidget _aswbp_text_popup))
  (Variables|/Game/Blueprints/Widgets/WBP_TextPopup.WBP_TextPopup_C|SetText _output_get (Variables|Default|GetTriggerText))
  (if (Variables|Default|GetShowing)
    (Default|Reveal (Variables|Default|GetNotificationWidget))))

(event Collision|EventActorBeginOverlap
  (params (OtherActor :type Actor%20Object%20Reference))
  ;[1 1 1] Hide and Reveal Widget
  (if (not (Variables|Default|GetShowing))
    (Default|Reveal (Variables|Default|GetNotificationWidget))
    (Variables|Default|SetShowing true)))

(event Collision|EventActorEndOverlap
  (params (OtherActor :type Actor%20Object%20Reference))
  ;[1 1 1] Hide and Reveal Widget
  (if (Variables|Default|GetShowing)
    (Default|Hide (Variables|Default|GetNotificationWidget))
    (Variables|Default|SetShowing false)))

(fn ConstructionScript)