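; Arena Blueprint that tracks a set of enemies and signals when all of them have died.
; On BeginPlay it counts EnemyArray and binds each enemy's OnDeath event to EnemyDestroyed.
; Each death decrements the count, and at zero or below it calls the OnCleared dispatcher and prints a debug string.
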(event Custom|EnemyDestroyed
  (bind _enemycount (Variables|Default|GetEnemyCount))
  (Math|Integer|DecrementInt _enemycount
    (:%20%20
      (if (<= _enemycount 0)
        (Default|CallOnCleared)
        (Development|PrintString "Hello")))))

(event EventBeginPlay
  (Variables|Default|SetEnemyCount (Utilities|Array|Length (Variables|Default|GetEnemyArray)))
  (for _array_element (Variables|Default|GetEnemyArray)
    (EventDispatchers|BindEventtoOnDeath _array_element (delegate Custom|EnemyDestroyed))))

(fn ConstructionScript)