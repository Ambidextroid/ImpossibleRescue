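; BP_InteractTriggerOpaque is an interaction trigger that shows a text popup when the player interacts with it.
; BeginPlay caches the WBP_TextPopup from its widget component and sets the trigger text.
; If the popup starts hidden, the component is made invisible for half a second while Hide runs.
; Interacted reveals the popup, and any actor's end overlap hides it, with a Showing flag preventing repeat calls.
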(event EventBeginPlay
  ;[1 1 1] Cache widget reference and set widget text
  (bind _aswbp_text_popup (Utilities|Casting|CastToWBP_TextPopup (UserInterface|GetWidget (Variables|Default|GetTextWidget))))
  (bind _output_get (Variables|Default|SetNotificationWidget _aswbp_text_popup))
  (Variables|/Game/Blueprints/Widgets/WBP_TextPopup.WBP_TextPopup_C|SetText _output_get (Variables|Default|GetTriggerText))
  (if (not (Variables|Default|GetShowing))
    (Rendering|SetVisibility (Variables|Default|GetTextWidget) false false)
    (Default|Hide (Variables|Default|GetNotificationWidget))
    (Utilities|FlowControl|Delay 0.5)
    (Rendering|SetVisibility (Variables|Default|GetTextWidget) true false)))

(event EventInteracted
  ;[1 1 1] If message not showing and player interacts, show the message
  (if (not (Variables|Default|GetShowing))
    (Default|Reveal (Variables|Default|GetNotificationWidget))
    (Variables|Default|SetShowing true)))

(event Collision|EventActorEndOverlap
  (params (OtherActor :type Actor%20Object%20Reference))
  ;[1 1 1] If player leaves vicinity and message still showing, hide it
  (if (Variables|Default|GetShowing)
    (Default|Hide (Variables|Default|GetNotificationWidget))
    (Variables|Default|SetShowing false)))

(fn ConstructionScript)