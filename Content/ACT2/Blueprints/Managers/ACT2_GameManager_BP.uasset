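; ACT2_GameManager_BP is a manager Blueprint for ACT2 that owns the player HUD and handles level restarts.
; On BeginPlay it creates the ACT2_HUD_Widget, adds it to the viewport and shows the mouse cursor.
; UpdateHealthOnHUD sets the health bar from a health value on a 100-point scale.
; RestartLevel reopens the current level by looking up its name.
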(event EventBeginPlay
  (bind _returnvalue (UserInterface|CreateWidget "/Game/ACT2/Blueprints/UI/ACT2_HUD_Widget.ACT2_HUD_Widget_C"))
  (bind _output_get (Variables|Default|SetHUD _returnvalue))
  (UserInterface|Viewport|AddtoViewport _output_get 0)
  (Variables|/Script/Engine.PlayerController|SetbShowMouseCursor (Game|GetPlayerController 0) true))

(fn ConstructionScript)

(fn RestartLevel
  ;[1 1 1] Restarting current level. Could use a refactor, not keen on doing it by name
  (bind _returnvalue (Game|GetCurrentLevelName true))
  (Game|OpenLevel(byName) (Utilities|String|StringToName _returnvalue)))

(fn UpdateHealthonHUD
  (params (Health :type Integer))
  (Progress|SetPercent (Variables|/Game/ACT2/Blueprints/UI/ACT2_HUD_Widget.ACT2_HUD_Widget_C|GetHealthBar (Variables|Default|GetHUD)) (/ (Math|Conversions|ToFloat(Integer) Health) 1e+02)))