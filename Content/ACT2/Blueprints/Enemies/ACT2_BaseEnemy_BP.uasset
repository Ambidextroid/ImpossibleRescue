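; Base enemy for Act 2 that patrols random navmesh points, chases the player, takes damage and is destroyed at zero health.
; Tick distance checks start pursuit when the player enters range and set HasSeenPlayer, which keeps later re-checks pursuing.
; AI MoveTo drives both states, with cleared-on-switch timers pacing patrol waits and pursuit re-checks, and an empty ReachedPlayer hook on arrival.
; Optional sphere-overlap contact sends damage and horizontal knockback through KnockbackMessage.
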(event OnComponentBeginOverlap(Sphere)
  (params (OverlappedComponent :type Primitive%20Component%20Object%20Reference) (OtherActor :type Actor%20Object%20Reference) (OtherComp :type Primitive%20Component%20Object%20Reference) (OtherBodyIndex :type Integer) (bFromSweep :type Boolean) (SweepResult :type Hit%20Result%20Structure%20%28by%20ref%29))
  ;[1 1 1] If enemy has collision damage set (for knockback), then deals knockback damage and force
  (if (Variables|Collision|GetHasCollisionDamage)
    (bind _direction (CallFunction|GetKnockbackDir))
    (Class|ACT2DamageInterface|Knockback(Message) OtherActor _direction (Variables|Collision|GetKnockbackHeight) (Variables|Collision|GetKnockbackDistance) (Variables|Collision|GetCollisionDamage))))

(event Custom|Event%20PursuePlayer
  ;[1 1 1] Pursue event, called when player enters the range of the enemy, then moves to within the specified distance of the player. Afterwards, checks whether it should resume pursuit, or return to patrolling
  (CallFunction|ClearTimerHandles)
  (Variables|Default|SetState "NewEnumerator2")
  (AI|AIMoveTo (AI|GetAIController self) "0, 0, 0" (Variables|Player|GetPlayer) (Variables|Player|GetPlayerStopDistance) "Default" "Default" true true
    (:then
      (bind _returnvalue (Utilities|Time|SetTimerbyFunctionName 0 "PursueOrPatrol" (Variables|Movement|GetResumePursuitDelay)))
      (Variables|Default|SetPursuitTimerHandle _returnvalue))
    (:OnMoveFinished
      (CallFunction|ReachedPlayer))))

(event Custom|Event%20Patrol
  ;[1 1 1] Patrol logic, patrols to a random point within the patrol radius, waits for a random time, then recalls the event
  (CallFunction|ClearTimerHandles)
  (Variables|Default|SetState "NewEnumerator1")
  (bind _nextpatrolpoint (CallFunction|FindNextPatrolPoint))
  (AI|AIMoveTo (AI|GetAIController self) _nextpatrolpoint 0 -1.0 "Default" "Default" true true
    (:OnMoveFinished
      (bind _returnvalue (Utilities|Time|SetTimerbyEvent (delegate Custom|Event%20Patrol) (Math|Random|RandomFloatinRange (Variables|Patrol|GetPatrolDelayMin) (Variables|Patrol|GetPatrolDelayMax))))
      (Variables|Default|SetPatrolTimerHandle _returnvalue))))

(event EventTick
  (params (DeltaSeconds :type Float%20%28single-precision%29))
  ;[1 1 1] Event tick, currently used to check whether player is in distance
  (CallFunction|TrackPlayerDistance))

(event EventDamage
  (params (Damage :type Integer))
  (CallFunction|IncomingDamage Damage))

(event EventBeginPlay
  ;[1 1 1] Getting player reference, then calling the patrol event to begin patrolling
  (CallFunction|RetrievePlayerRef)
  (if (Variables|Patrol|GetCanPatrol)
    (CallFunction|EventPatrol)))

(fn ConstructionScript)

(fn IsPlayerinDetectionRange
  (return (<= (Math|Vector|Distance(Vector) (Transformation|GetActorLocation (Variables|Player|GetPlayer)) (Transformation|GetActorLocation)) (Variables|Player|GetPlayerDetectionDist))))

(fn RetrievePlayerRef
  (Variables|Player|SetPlayer (Game|Player|GetPlayerPawn 0)))

(fn GetKnockbackDir
  (bind _returnvalue (Transformation|GetActorLocation))
  (bind _player (Variables|Player|GetPlayer))
  (bind _returnvalue_2 (Transformation|GetActorLocation _player))
  (bind _returnvalue_3 (Math|Vector|GetUnitDirection(Vector) _returnvalue _returnvalue_2))
  ;[1 1 1] Getting dir from enemy to player, ignoring the z, then returning result
  (return (Math|Vector|Normalize (Math|Vector|MakeVector (.x _returnvalue_3) (.y _returnvalue_3) 0.0))))

(fn FindNextPatrolPoint
  ;[1 1 1] Find random point in navmesh within specified radius
  (return (.RandomLocation (Class|NavigationSystemV1|GetRandomPointinNavigableRadius (Transformation|GetActorLocation) (Variables|Patrol|GetPatrolRadius) 0 0))))

(fn ClearTimerHandles
  ;[1 1 1] Clearing timer handles to avoid functions being called out of turn
  (Utilities|Time|ClearandInvalidateTimerbyHandle (Variables|Default|GetPatrolTimerHandle))
  (Utilities|Time|ClearandInvalidateTimerbyHandle (Variables|Default|GetPursuitTimerHandle)))

(fn ReachedPlayer)

(fn PursueorPatrol
  ;[1 1 1] Determining whether to resume pursuit or return to patrol, based on if the player is still in range
  (bind _isplayerindetectionrange (CallFunction|IsPlayerinDetectionRange))
  (if (or _isplayerindetectionrange (Variables|Player|GetHasSeenPlayer))
    (CallFunction|EventPursuePlayer)
    (elif (Variables|Patrol|GetCanPatrol)
      (CallFunction|EventPatrol))))

(fn TrackPlayerDistance
  ;[1 1 1] Tracking if the player is in range, and if so and they weren't previously in range, calling the pursue event
  (bind _isplayerindetectionrange (CallFunction|IsPlayerinDetectionRange))
  (if (and _isplayerindetectionrange (not (Variables|Player|GetPlayerPreviouslyInRange)))
    (Variables|Player|SetPlayerPreviouslyInRange true)
    (CallFunction|EventPursuePlayer)
    (Variables|Player|SetHasSeenPlayer true)
    (elif (not _isplayerindetectionrange)
      (Variables|Player|SetPlayerPreviouslyInRange false))))

(fn IncomingDamage
  (params (Damage :type Integer))
  (if (<= (- (Variables|Default|GetHealth) Damage) 0)
    (Variables|Default|SetHealth 0)
    (CallFunction|Death)
    (else
      (Variables|Default|SetHealth (- (Variables|Default|GetHealth) Damage)))))

(fn Death
  (Actor|DestroyActor))