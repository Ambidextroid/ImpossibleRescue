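; High-tier enemy for Act 2 that fires bursts of projectiles at the player upon reaching them.
; ReachedPlayer starts a looping timer that spawns projectiles aimed along the normalized X/Y direction to the player, and schedules PursueOrPatrol after a delay.
; Each shot increments a counter, which Tick checks to clear the timer and reset once the burst size is reached.
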(event EventBeginPlay
  (|CallParentFunction) ; This node is disabled and will not be called.\nDrag off pins to build functionality.
)

(event Collision|EventActorBeginOverlap
  (params (OtherActor :type Actor%20Object%20Reference)))

(event EventTick
  (params (DeltaSeconds :type Float%20%28single-precision%29))
  (|CallParentFunction DeltaSeconds)
  (CallFunction|TrackBurstShots))

(fn ConstructionScript
  (|CallParentFunction))

(fn ReachedPlayer
  (CallFunction|BurstFire)
  (Utilities|Time|SetTimerbyFunctionName 0 "PursueOrPatrol" (Variables|Default|GetResumePursuitDelay)))

(fn FireProjectile
  (bind _returnvalue (Transformation|GetActorLocation))
  (bind _player (Variables|Default|GetPlayer))
  (bind _returnvalue_2 (Transformation|GetActorLocation _player))
  (bind _returnvalue_3 (Math|Vector|GetUnitDirection(Vector) _returnvalue _returnvalue_2))
  (bind _returnvalue_4 (Game|SpawnActorfromClass "/Game/ACT2/Blueprints/Projectiles/ACT2_EnemyProjectile_BP.ACT2_EnemyProjectile_BP_C" (Math|Transform|MakeTransform _returnvalue "0, 0, 0" "1,1,1") "Undefined" 0 0))
  (Default|SetuptoFire _returnvalue_4 (Math|Vector|Normalize (Math|Vector|MakeVector (.x _returnvalue_3) (.y _returnvalue_3) 0.0)) (Variables|Default|GetProjectileDamage) self))

(fn FireBurstShot
  (CallFunction|FireProjectile)
  (Math|Integer|IncrementInt (Variables|Default|GetShotsInCurrentBurst)))

(fn BurstFire
  (bind _returnvalue (Utilities|Time|SetTimerbyFunctionName 0 "FireBurstShot" (Variables|Default|GetBurstFireInterval) true))
  (Variables|Default|SetBurstFireTimerHandle _returnvalue))

(fn TrackBurstShots
  (if (>= (Variables|Default|GetShotsInCurrentBurst) (Variables|Default|GetShotsPerBurst))
    (Utilities|Time|ClearandInvalidateTimerbyHandle (Variables|Default|GetBurstFireTimerHandle))
    (Variables|Default|SetShotsInCurrentBurst 0)))