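; Virus enemy Blueprint for ACT2, apparently a 2D variant, that moves toward the player through its AI controller.
; InitialPlayerDetection issues a MoveToActor on Player with partial paths and stop-on-overlap disabled, then prints a debug string.
; Movement is an empty stub, BeginPlay and construction only call the parent, and nothing in this file calls the detection function.
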(event EventBeginPlay
  (|CallParentFunction))

(event Collision|EventActorBeginOverlap
  (params (OtherActor :type Actor%20Object%20Reference))
  (|CallParentFunction OtherActor) ; This node is disabled and will not be called.\nDrag off pins to build functionality.
)

(event EventTick
  (params (DeltaSeconds :type Float%20%28single-precision%29))
  (|CallParentFunction DeltaSeconds) ; This node is disabled and will not be called.\nDrag off pins to build functionality.
)

(fn ConstructionScript
  (|CallParentFunction))

(fn Movement)

(fn InitialPlayerDetection
  (AI|Navigation|MovetoActor (AI|GetAIController self) (Variables|Default|GetPlayer) -1.0 false true true 0 false)
  (Development|PrintString "MoveTo"))