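; Enemy-fired projectile Blueprint that damages what it hits while ignoring Enemy_2DBP, building on a parent projectile class.
; CheckForTarget calls ShouldIgnoreCollision with Enemy_2DBP as the class to skip.
; For any other target it sends the ProjectileCollisionMessage interface call with Damage, then destroys itself.
; The event graph and construction script only call the parent, with overlap and tick disabled.
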(event EventBeginPlay
  (|CallParentFunction))

(event Collision|EventActorBeginOverlap
  (params (OtherActor :type Actor%20Object%20Reference))
  (|CallParentFunction OtherActor) ; This node is disabled and will not be called.\nDrag off pins to build functionality.
)

(event EventTick
  (params (DeltaSeconds :type Float%20%28single-precision%29))
  (|CallParentFunction DeltaSeconds) ; This node is disabled and will not be called.\nDrag off pins to build functionality.
)

(fn ConstructionScript
  (|CallParentFunction))

(fn CheckforTarget
  (params (Collision%20Target :type Actor%20Object%20Reference))
  ;[1 1 1] Check whether collision should be ignored
  (bind _shouldignore (CallFunction|ShouldIgnoreCollision Collision%20Target "/Game/ACT2/Blueprints/Enemies/Enemy_2DBP.Enemy_2DBP_C"))
  (if (not _shouldignore)
    ;[1 1 1] Attempt interface function on target, then destroy this projectile
    (Class|ACT2DamageInterface|ProjectileCollision(Message) Collision%20Target (Variables|Default|GetDamage))
    (Actor|DestroyActor)))