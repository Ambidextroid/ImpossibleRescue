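; Base 2D projectile Blueprint that flies in a set direction and destroys itself on any actor overlap or when its lifetime expires.
; SetupToFire stores damage and direction, rotating the actor by a look-at pitch remapped for leftward movement.
; Tick moves it without sweep and counts lifetime.
; ShouldIgnoreCollision can filter projectiles and a given class, but the default CheckForTarget neither calls it nor applies damage.
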(event Collision|EventActorBeginOverlap
  (params (OtherActor :type Actor%20Object%20Reference))
  ;[1 1 1] Get collision object, then pass the object to the function
  (CallFunction|CheckforTarget OtherActor))

(event EventTick
  (params (DeltaSeconds :type Float%20%28single-precision%29))
  ;[1 1 1] Movement update
  (CallFunction|Move)
  ;[1 1 1] Check if the projectile's lifetime has expired, then destroy if so
  (CallFunction|LifetimeCheck))

(fn ConstructionScript)

(fn Move
  ;[1 1 1] Add the movement calculation to the current position, then set
  (Transformation|SetActorLocation (+ (Transformation|GetActorLocation) (* (Variables|Default|GetMoveDir) (* (Variables|Default|GetSpeed) (Utilities|Time|GetWorldDeltaSeconds)))) false false))

(fn SetDir
  (params (Direction :type Vector))
  (bind _returnvalue (Transformation|GetActorLocation))
  ;[1 1 1] Get angle for rotation based on direction of movement
  (bind _output_get (Variables|Default|SetMoveDir (* Direction 1.0)))
  ;[1 1 1] Translate angles into 0 to 360 for correct rotation values
  (bind _angle_out (CallFunction|TranslateAngle (.pitch (Math|Rotator|FindLookatRotation _returnvalue (+ _returnvalue _output_get)))))
  (Transformation|SetActorRotation (Math|Rotator|MakeRotator 0.0 _angle_out 0.0)))

(fn LifetimeCheck
  ;[1 1 1] Count the lifetime of the projectile using delta time, once lifetime has passed max, destroy this actor
  (bind _output_get (Variables|Default|SetCurrentLifetime (+ (Variables|Default|GetCurrentLifetime) (Utilities|Time|GetWorldDeltaSeconds))))
  (if (>= _output_get (Variables|Default|GetMaxLifetime))
    (Actor|DestroyActor)))

(fn TranslateAngle
  (params (Angle%20In :type Float%20%28single-precision%29))
  ;[1 1 1] Unreal was giving me angles in -90 to 90 degrees, which was breaking projectile rotation.
  ; This function translates that into 0 to 360 degrees.
  (if (>= (.x (Variables|Default|GetMoveDir)) 0.0)
    (return Angle%20In)
    (else
      (return (- 3.6e+02 Angle%20In)))))

(fn CheckforTarget
  (params (Collision%20Target :type Actor%20Object%20Reference))
  ;[1 1 1] Default collision for base projectile class,
  ; destroy actor on any collision
  (Actor|DestroyActor))

(fn SetDamage
  (params (Damage :type Integer))
  ;[1 1 1] Function for setting the damage of the projectile
  (Variables|Default|SetDamage Damage))

(fn SetuptoFire
  (params (Direction :type Vector) (Damage :type Integer))
  (CallFunction|SetDir Direction)
  (CallFunction|SetDamage Damage))

(fn ShouldIgnoreCollision
  (params (CollisionTarget :type Actor%20Object%20Reference) (ClassToIgnore :type Actor%20Class%20Reference))
  (bind _returnvalue (Utilities|GetClass CollisionTarget))
  ;[1 1 1] Ignore if collision is another projectile
  (if (Utilities|ClassIsChildOf _returnvalue "Projectile_2DBP_C")
    _
    (else
      ;[1 1 1] Ignore if collision is from the same class it was fired from
      (if (Utilities|ClassIsChildOf _returnvalue ClassToIgnore)
        _
        (else
          (return false)))))
  (return true))