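; BP_DaughterModel is an actor for the daughter's skeletal mesh that hovers vertically in place.
; On BeginPlay it stores the mesh's world location and plays a slowed timeline.
; Each update adds the scaled timeline track to the starting Z while holding X and Y fixed.
; Overlap, Tick and the construction script contain no logic.
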(event EventBeginPlay
  ;[1 1 1] Hover up and down in place
  (Variables|Default|Setstartloc (Transformation|GetWorldLocation (Variables|SkeletalMeshActor|GetSkeletalMeshComponent)))
  (Components|Timeline|SetPlayRate (Variables|Default|GetTimeline_0) 0.15)
  (bind _newtrack_0 (Timeline|Timeline_0 Play)
    (:Update
      (Transformation|SetWorldLocation (Variables|SkeletalMeshActor|GetSkeletalMeshComponent) (Math|Vector|MakeVector (.X (Math|Vector|BreakVector (Variables|Default|Getstartloc))) (.Y (Math|Vector|BreakVector (Variables|Default|Getstartloc))) (+ (* _newtrack_0 2e+01) (.Z (Math|Vector|BreakVector (Variables|Default|Getstartloc))))) false false))))

(event Collision|EventActorBeginOverlap
  (params (OtherActor :type Actor%20Object%20Reference)))

(event EventTick
  (params (DeltaSeconds :type Float%20%28single-precision%29)))

(fn ConstructionScript)